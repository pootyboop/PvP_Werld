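; Campfire actor that damages actors standing in the fire and heals those around it.
; Tick, throttled by a Delay, asks BP_MainGameState to spawn a small damage AOE and a larger heal AOE, neither requiring line of sight.
; Damaged actors are recorded so the heal skips them, then the list is cleared.
; Both amounts scale by Tick's DeltaSeconds despite the delayed pulse.
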(event `self.ReceiveTick`
  (params (DeltaSeconds :type "Float (single-precision)"))
  (bind _returnvalue (`self.K2_GetActorLocation`))
  (`KismetSystemLibrary.Delay` 0.3)
  (bind _asbp_main_game_state (cast `/Game/Loadouts/Characters/BaseClass/BP_MainGameState` (`GameplayStatics.GetGameState`)))
  (`/Game/Loadouts/Characters/BaseClass/BP_MainGameState.Spawn AOE` _asbp_main_game_state _returnvalue 32.0 false self (delegate `Damage AOE`) 0.0 (struct :`R` 1.0 :`G` 1.0 :`B` 1.0 :`A` 1.0))
  (`/Game/Loadouts/Characters/BaseClass/BP_MainGameState.Spawn AOE` _asbp_main_game_state _returnvalue 384.0 false null (delegate `Heal AOE`) 0.0 (struct :`R` 1.0 :`G` 1.0 :`B` 1.0 :`A` 1.0))
  (`KismetArrayLibrary.Array_Clear` (`self.Damaged Players`)))

(event `Damage AOE`
  (params (`Hit Actor` :type "Actor Object Reference"))
  (message `/Game/HealthInterface/BPI_HealthInterface.Damage` `Hit Actor` (make `/Game/HealthInterface/Dmg` (* 100 (stale `self.ReceiveTick` DeltaSeconds)) "NewEnumerator6" null self))
  (`KismetArrayLibrary.Array_Add` (`self.Damaged Players`) `Hit Actor`))

(event `Heal AOE`
  (params (`Hit Actor` :type "Actor Object Reference"))
  (if (not (`KismetArrayLibrary.Array_Contains` (`self.Damaged Players`) `Hit Actor`))
    (message `/Game/HealthInterface/BPI_HealthInterface.Heal` `Hit Actor` (* 100 (stale `self.ReceiveTick` DeltaSeconds)))))

(fn `UserConstructionScript`
  (`parent.UserConstructionScript`))