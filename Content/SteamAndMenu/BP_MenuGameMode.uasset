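; BP_MenuGameMode is the menu game mode that gives each starting player a menu pawn.
; HandleStartingNewPlayer records the controller in a unique player list, then spawns a BP_MenuPawn at a fixed transform and has that controller possess it.
; It also copies the max player count and server name from the Steam game instance, fetched through a message call.
; PostLogin and the construction script are empty.
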(event `self.HandleStartingNewPlayer`
  (params (NewPlayer :type "PlayerController Object Reference"))
  (bind _output_get (set `self.ConnectedPlayer` NewPlayer))
  (`KismetArrayLibrary.Array_AddUnique` (`self.Players`) _output_get)
  (bind _game_instance (message `/Game/SteamAndMenu/BPI_GameInstance.SteamGameInstanceRef` (`GameplayStatics.GetGameInstance`)))
  (set `self.Max Players` (`/Game/SteamAndMenu/SteamGameInstance.maxPlayers` _game_instance))
  (set `self.Server Name` (`/Game/SteamAndMenu/SteamGameInstance.Server Name` _game_instance))
  (bind _returnvalue (`|SpawnActorFromClass` "/Game/SteamAndMenu/BP_MenuPawn.BP_MenuPawn_C" (`KismetMathLibrary.MakeTransform` (-699.0 31.0 116.0) (struct :`Yaw` 5.0)) "Undefined" "OverrideRootScale" null null))
  (`Controller.Possess` _output_get _returnvalue))

(event `self.K2_PostLogin`
  (params (NewPlayer :type "PlayerController Object Reference")))

(fn `UserConstructionScript`)