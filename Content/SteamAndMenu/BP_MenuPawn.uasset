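; Menu pawn that runs the main menu and party lobby for a Steam-enabled game.
; On BeginPlay the local pawn creates W_MainMenu with the saved color and sets the Steam nickname.
; After a delay it passes saved name, color and level through Server-to-Multi events, adding an entry to the local menu's party list.
; It also opens CloudIslands through SteamGameInstance on game start and slides the camera with a reversible timeline.
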(event `Set Main Menu Server`
  (params (`Main Menu` :type "/Game/UI/Menu/MainMenu/W_MainMenu Object Reference"))
  (set `self.Main Menu` `Main Menu`)
  (`KismetSystemLibrary.PrintString` (`KismetSystemLibrary.GetDisplayName` (`self.Main Menu`)) true true (struct :`G` 0.122397 :`B` 1.0 :`A` 1.0)))

(event `self.ReceiveBeginPlay`
  (bind _save_game (`/Game/BPFunctionLibrary.Get Save Game`))
  (bind _returnvalue (`GameplayStatics.GetPlayerController` 0))
  (bind _playernickname (`AdvancedIdentityLibrary.GetPlayerNickname` (`AdvancedSessionsLibrary.GetUniqueNetID` (`GameplayStatics.GetPlayerController` 0))))
  (`|ExecutionSequence`
    (:`then_0`
      (if (`self.IsLocallyControlled`)
        (bind _returnvalue_2 (`|CreateWidget` "/Game/UI/Menu/MainMenu/W_MainMenu.W_MainMenu_C" (`GameplayStatics.GetPlayerController` 0) (`/Game/Saving/BP_SaveGame.Color` (`/Game/BPFunctionLibrary.Get Save Game`))))
        (set `self.Main Menu` _returnvalue_2)
        (`UserWidget.AddToViewport` (`self.Main Menu`) 0)
        (set `PlayerController.bShowMouseCursor` true _returnvalue)
        (`WidgetBlueprintLibrary.SetInputMode_UIOnlyEx` _returnvalue (`self.Main Menu`))
        (if (`AdvancedSessionsLibrary.HasOnlineSubsystem` "STEAM")
          (`KismetSystemLibrary.Delay` 0.2)
          (`/Game/UI/Menu/MainMenu/W_MainMenu.SetPlayerName` (`self.Main Menu`) (`KismetTextLibrary.Conv_StringToText` (`KismetMathLibrary.SelectString` "Offline Player" _playernickname (`KismetStringLibrary.IsEmpty` _playernickname)))))))
    (:`then_1`
      (`KismetSystemLibrary.Delay` 1.0)
      (if (`self.IsLocallyControlled`)
        (`self.Join Party List Server` self (`KismetTextLibrary.Conv_StringToText` (`/Game/Saving/BP_SaveGame.Player Name` _save_game)) (`/Game/Saving/BP_SaveGame.Color` _save_game) (`/Game/Saving/BP_SaveGame.Level` _save_game))))))

(event `Join Party List Server`
  (params (Target :type "Self Object Reference") (PlayerName :type Text) (Color :type "LinearColor Structure") (Lvl :type Integer))
  (`self.Join Party List Multi` Target PlayerName Color Lvl))

(event `Join Party List Multi`
  (params (PlayerName :type Text) (Color :type "LinearColor Structure") (Lvl :type Integer))
  (bind _asbp_menu_pawn (cast `/Game/SteamAndMenu/BP_MenuPawn` (`Controller.K2_GetPawn` (`GameplayStatics.GetPlayerController` 0)) :!pure true))
  (bind _returnvalue (`|CreateWidget` "/Game/UI/Menu/MainMenu/W_PartyPlayerName.W_PartyPlayerName_C" (`GameplayStatics.GetPlayerController` 0) PlayerName Color Lvl))
  (bind _main_menu (`/Game/SteamAndMenu/BP_MenuPawn.Main Menu` _asbp_menu_pawn)
    (:`then`
      (if (`|EnumEquality` (`Widget.GetVisibility` (`/Game/UI/Menu/MainMenu/W_MainMenu.PlayerList` _main_menu)) "Hidden")
        (`Widget.SetVisibility` (`/Game/UI/Menu/MainMenu/W_MainMenu.PlayerList` _main_menu) "Visible"))
      (`PanelWidget.AddChild` (`/Game/UI/Menu/MainMenu/W_MainMenu.PARTY` (`/Game/SteamAndMenu/BP_MenuPawn.Main Menu` _asbp_menu_pawn)) _returnvalue))
    (:`else`
      (`KismetSystemLibrary.PrintString` "invalid main menu ref on menupawn"))))

(event `self.ReceiveEndPlay`
  (params (EndPlayReason :type "EEndPlayReason Enum" :default "Destroyed"))
  (bind _main_menu (`self.Main Menu`)
    (:`then`
      (`Widget.RemoveFromParent` _main_menu))
    (:`else`)))

(event `Key|K`
  (params (Key :type "Key Structure"))
  (:`Pressed`
    (`KismetSystemLibrary.PrintString` "K")))

(event `Start Game`
  (`self.Start Game Server`))

(event `Start Game Server`
  (`/Game/SteamAndMenu/SteamGameInstance.Open Level` (cast `/Game/SteamAndMenu/SteamGameInstance` (`GameplayStatics.GetGameInstance`) :!pure true) "CloudIslands"))

(event `Start Camera Move`
  (bind (_direction _camera_position) (`Timeline|Camera Move Timeline` :!via `PlayFromStart` :!label _label)
    (:`Update`
      (`SceneComponent.K2_SetRelativeLocation` (`self.Camera`) (`KismetMathLibrary.MakeVector` 0.0 _camera_position) false false))))

(event `End Camera Move`
  (goto _label :!via `ReverseFromEnd`))

(fn `UserConstructionScript`)