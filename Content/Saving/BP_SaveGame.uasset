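; SaveGame object that stores the player's weapon loadouts and the index of the equipped one.
; Helpers add, remove, swap, edit or equip loadouts, immediately writing the object to a single fixed save slot.
; A repair pass pads both weapons' mod-equipped arrays with false toward the data table row count, saving after each weapon.
; The padding loop compares the shrinking shortfall to the growing array length, so it can stop short.
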(fn `Add New Loadout and Save`
  (params (`New Loadout` :type "/Game/Loadouts/sLoadout Structure (by ref)"))
  (returns (`New Loadout Index` :type Integer))
  (bind _returnvalue (`KismetArrayLibrary.Array_Add` (`self.Loadouts`) `New Loadout`))
  (`self.Save`)
  (return _returnvalue))

(fn `Equip Loadout by Index and Save`
  (params (Index :type Integer))
  (set `self.Equipped Loadout Index` Index)
  (`self.Save`))

(fn `Fix All Loadout Mod Counts`
  (returns (`Save Game` :type "/Game/Saving/BP_SaveGame Object Reference"))
  (locals (`Total Mod Count` :type Integer :default 0))
  (bind _outrownames (`DataTableFunctionLibrary.GetDataTableRowNames` null))
  (set `local.Total Mod Count` (`KismetArrayLibrary.Array_Length` _outrownames))
  (for (_array_element _array_index) (`self.Loadouts`)
    (bind (_loadoutname _loadoutcolor _character _weapon1 _weapon1mods _weapon1skins _weapon2 _weapon2mods) (break `/Game/Loadouts/sLoadout` _array_element))
    (bind _return (`self.Fix Mod Array Count` _weapon1mods (`local.Total Mod Count`)))
    (bind _structout (setmembers `/Game/Loadouts/sLoadout` :`StructRef` _array_element :`Weapon 1 Mods` _return))
    (bind _updated_loadout (`self.Set Loadout Info And Save` _structout _array_index))
    (bind _return_2 (`self.Fix Mod Array Count` _weapon2mods (`local.Total Mod Count`)))
    (bind _structout_2 (setmembers `/Game/Loadouts/sLoadout` :`StructRef` _updated_loadout :`Weapon 2 Mods` _return_2))
    (`self.Set Loadout Info And Save` _structout_2 _array_index))
  (return self))

(fn `Fix Mod Array Count`
  (params (ModLevels :type "/Game/Loadouts/Weapons/Mods/ModLevels Structure (by ref)") (`Total Mod Count` :type Integer))
  (returns (Return :type "/Game/Loadouts/Weapons/Mods/ModLevels Structure (by ref)"))
  (locals (Difference :type Integer :default 0))
  (bind _modlevels_equipped (break `/Game/Loadouts/Weapons/Mods/ModLevels` (`local.ModLevels`)))
  (bind _returnvalue (`KismetArrayLibrary.Array_Length` (`.Equipped_11_5E7168F145FFCB405FD71A8D5073BBBC` (break `/Game/Loadouts/Weapons/Mods/ModLevels` ModLevels))))
  (bind _returnvalue_2 (- `Total Mod Count` _returnvalue))
  (if (> _returnvalue_2 0)
    (set `local.Difference` _returnvalue_2)
    (while (> (`local.Difference`) _returnvalue)
      (`/Engine/EditorBlueprintResources/StandardMacros.DecrementInt` (`local.Difference`)
        (:`  `
          (`KismetArrayLibrary.Array_Add` _modlevels_equipped))))
    (return (`local.ModLevels`))
    (else
      (return (`local.ModLevels`)))))

(fn `Get Currently Equipped Loadout`
  (returns (Loadout :type "/Game/Loadouts/sLoadout Structure (by ref)"))
  (return (`|GetArrayItem` (`self.Loadouts`) (`self.Equipped Loadout Index`))))

(fn `Remove Loadout by Index and Save`
  (params (Index :type Integer))
  (bind _loadouts (`self.Loadouts`))
  (`KismetArrayLibrary.Array_RemoveItem` _loadouts (`|GetArrayItem` _loadouts Index))
  (`self.Save`))

(fn `Save`
  (`GameplayStatics.SaveGameToSlot` self "Save"))

(fn `Set Loadout Info And Save`
  (params (Loadout :type "/Game/Loadouts/sLoadout Structure") (`Loadout Index` :type Integer))
  (returns (`Updated Loadout` :type "/Game/Loadouts/sLoadout Structure (by ref)"))
  (`KismetArrayLibrary.Array_Set` (`self.Loadouts`) `Loadout Index` Loadout)
  (`self.Save`)
  (return Loadout))

(fn `Swap Loadout Locations and Save`
  (params (`First Loadout Index` :type Integer) (`Second Loadout Index` :type Integer))
  (locals (Temp :type "/Game/Loadouts/sLoadout Structure"))
  (bind _loadouts (`self.Loadouts`))
  (bind _loadouts_2 (`self.Loadouts`))
  (set `local.Temp` (`|GetArrayItem` _loadouts_2 `Second Loadout Index`) :!pinned true) ; Set Temp to 2nd
  (`KismetArrayLibrary.Array_Set` _loadouts `Second Loadout Index` (`|GetArrayItem` _loadouts_2 `First Loadout Index`) :!pinned true) ; Set 2nd to 1st
  (`KismetArrayLibrary.Array_Set` _loadouts `First Loadout Index` (`local.Temp`) :!pinned true) ; Set 1st to temp
  (`self.Save`))