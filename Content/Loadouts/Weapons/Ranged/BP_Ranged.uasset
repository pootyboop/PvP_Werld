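; BP_Ranged is a ranged loadout weapon that handles firing, ammo, kickback, reload animation and headshot-multiplier mods.
; Fire branches on fire type, with Blast and Burst looping on a delay, into line-trace hits damaged through a server event or spawned BP_Projectiles.
; Each shot decrements ammo, shows muzzle flash and pushes the player.
; Projectiles spawn locally, then replicate via server and multicast with shared inaccuracy vectors, skipping the shooter.
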(event Custom|Kick%20Server
  (params (Player :type BP%20Character%20Base%20Object%20Reference) (Velocity :type Vector))
  (Physics|AddForce (Variables|/Script/Engine.Character|GetCharacterMovement Player) Velocity))

(event Custom|Fire%20Kick
  (params (Player :type BP%20Character%20Base%20Object%20Reference))
  (bind _ads__ (Variables|/Game/Loadouts/Characters/BaseClass/BP_CharacterBase.BP_CharacterBase_C|GetADS%20%25 Player))
  (bind _movementstate (Variables|/Game/Loadouts/Characters/BaseClass/BP_CharacterBase.BP_CharacterBase_C|GetMovementState Player))
  (bind _kick (Variables|WeaponInformation|Firing/Handling|GetKick))
  (bind _shots_per_click (Variables|WeaponInformation|Firing/Handling|GetShots%20per%20Click))
  (bind _camera (Variables|/Game/Loadouts/Characters/BaseClass/BP_CharacterBase.BP_CharacterBase_C|GetCamera Player))
  (bind _returnvalue (/ _ads__ 5.0))
  (bind _returnvalue_2 (Math|Conversions|ToFloat(Integer) _shots_per_click))
  (bind _returnvalue_3 (Math|Vector|GetForwardVector _camera))
  (bind _returnvalue_4 (Utilities|Enum|Equal(Enum) _movementstate "NewEnumerator1"))
  (bind _returnvalue_5 (/ _kick _returnvalue_2))
  (bind _returnvalue_6 (Math|Integer|SelectInt -200000 -400000 _returnvalue_4))
  (bind _returnvalue_7 (+ _returnvalue 1.0))
  (bind _returnvalue_8 (* _returnvalue_6 _returnvalue_5))
  (bind _returnvalue_9 (/ _returnvalue_8 _returnvalue_7))
  (bind _returnvalue_10 (Math|Float|SelectFloat _returnvalue_9 _returnvalue_8 false))
  (bind _returnvalue_11 (* _returnvalue_3 _returnvalue_10))
  (Physics|AddForce (Variables|/Script/Engine.Character|GetCharacterMovement Player) _returnvalue_11)
  (CallFunction|KickServer Player _returnvalue_11))

(event Custom|Spawn%20Projectile%20Server
  (params (Player :type BP%20Character%20Base%20Object%20Reference) (Camera :type Scene%20Component%20Object%20Reference) (Camera%20Transform :type Transform%20%28by%20ref%29) (Projectile%20Velocity%20Modifier%20%28+/-%29 :type Float%20%28single-precision%29) (Consistent%20Inaccuracy%20Vector :type Vector) (Combustion%20Rifle%20Consistent%20Inaccuracy%20Vectors :type Array%20of%20Vectors) (Fire%20from%20Location :type Vector))
  ;[1 0.2666 0] Projectile
  (CallFunction|SpawnProjectileMulti Player Camera Camera%20Transform Projectile%20Velocity%20Modifier%20%28+/-%29 Consistent%20Inaccuracy%20Vector Combustion%20Rifle%20Consistent%20Inaccuracy%20Vectors Fire%20from%20Location))

(event Custom|Spawn%20Projectile/Raytrace%20and%20Effects
  (params (Player :type BP%20Character%20Base%20Object%20Reference) (Camera :type Camera%20Component%20Object%20Reference) (Camera%20Transform :type Transform) (Projectile%20Velocity%20Modifier%20%28+/-%29 :type Float%20%28single-precision%29) (Shots%20to%20Fire :type Integer) (Fire%20from%20Location :type Vector))
  (bind (_location _rotation) (Math|Transform|BreakTransform Camera%20Transform))
  (Utilities|SwitchFireType
    (:Semi
      _)
    (:Automatic
      _)
    (:Blast
      (bind _output_get (Variables|Private|SetShots%20to%20Fire Shots%20to%20Fire :!label _label))
      (Utilities|ForLoopwithDelay 1 _output_get (Variables|WeaponInformation|Firing/Handling|GetBurst/Blast%20Delay)
        (:Loop%20Body
          _)))
    (:Burst
      (goto _label)))
  (if (Variables|WeaponInformation|Projectiles|GetisRaytraced)
    ;[0 0.6194 1] Raytrace
    (Utilities|FlowControl|Sequence
      (:then_0
        (bind (_outhit _returnvalue) (Collision|LineTraceByChannel _location (+ _location (* (Math|Vector|GetForwardVector _rotation) 10000)) "TraceTypeQuery1" true (Utilities|Array|MakeArray (Components|GetOwner) self) "ForDuration"))
        (if _returnvalue
          (CallFunction|OnHitAnything _outhit)
          (if (Utilities|DoesObjectImplementInterface (.HitActor (Collision|BreakHitResult _outhit)) "/Game/HealthInterface/BPI_HealthInterface.BPI_HealthInterface_C")
            (CallFunction|RangedDamageServer (.HitActor (Collision|BreakHitResult _outhit)) (Utilities|Struct|MakeDmg (* (* 2 (Variables|Default|GetAttack%20Damage)) (/ (.ranged (Variables|/Game/Loadouts/Characters/BaseClass/BP_CharacterBase.BP_CharacterBase_C|GetAttack Player)) 5.0)) "NewEnumerator2" (Game|GetPlayerController 0) self (Variables|Default|GetStatus%20Effects) (CallFunction|IsBoneHeadshot (.HitBoneName (Collision|BreakHitResult _outhit)))))
            (CallFunction|HitOpponent 0 (Utilities|Struct|MakeDmg (* (* 2 (Variables|Default|GetAttack%20Damage)) (/ (.ranged (Variables|/Game/Loadouts/Characters/BaseClass/BP_CharacterBase.BP_CharacterBase_C|GetAttack Player)) 5.0)) "NewEnumerator2" (Game|GetPlayerController 0) self (Variables|Default|GetStatus%20Effects) (CallFunction|IsBoneHeadshot (.HitBoneName (Collision|BreakHitResult _outhit))))))))
      (:then_1
        (Utilities|FlowControl|Sequence :!label _label_2
          (:then_0
            (CallFunction|DecrementandUpdateAmmo))
          (:then_1
            (Utilities|FlowControl|Sequence
              (:then_0
                (switch Utilities|FlowControl|Switch|SwitchonEWeaponClass (Variables|Default|GetWeapon%20Class)
                  (:NewEnumerator5
                    _)
                  (:NewEnumerator12
                    _)
                  (:NewEnumerator6
                    _)
                  (:NewEnumerator7
                    _)
                  (:NewEnumerator14
                    _))
                (Game|SpawnActorfromClass "/Game/Loadouts/Weapons/Ranged/Projectiles/BP_MuzzleFlash.BP_MuzzleFlash_C" (Math|Transform|MakeTransform Fire%20from%20Location "0, 0, 0" "1,1,1") "Undefined" 0 0))
              (:then_1
                (CallFunction|FireEffectsServer Player))))
          (:then_2
            (CallFunction|FireKick Player)))))
    (else
      ;[1 0.2666 0] Projectile
      (Utilities|FlowControl|Sequence
        (:then_0
          (bind _output_get_2 (Variables|Private|SetConsistent%20Inaccuracy%20Vector (CallFunction|CalculateInaccuracyVector)))
          (if (Utilities|Enum|Equal(Enum) (Variables|Default|GetWeapon%20Name) "NewEnumerator8")
            (bind _output_get_3 (Variables|Private|SetCombustion%20Rifle%20Inaccuracy%20Vectors (CallFunction|CalculateCombustionRifleInaccuracyVectors))))
          (CallFunction|SpawnProjectile Player Camera Camera%20Transform Projectile%20Velocity%20Modifier%20%28+/-%29 _output_get_2 _output_get_3 Fire%20from%20Location))
        (:then_1
          (CallFunction|SpawnProjectileServer Player Camera Camera%20Transform Projectile%20Velocity%20Modifier%20%28+/-%29 (Variables|Private|GetConsistent%20Inaccuracy%20Vector) (Variables|Private|GetCombustion%20Rifle%20Inaccuracy%20Vectors) Fire%20from%20Location))
        (:then_2
          (goto _label_2))))))

(event Custom|On%20Fire
  (bind _fire_animation (Variables|Default|GetFire%20Animation)
    (:then
      (bind _1st_person_weapon (Variables|/Game/Loadouts/Characters/BaseClass/BP_CharacterBase.BP_CharacterBase_C|Get1st%20Person%20Weapon (.AsBP%20Character%20Base (Utilities|Casting|CastToBP_CharacterBase (Components|GetOwner))))
        (:then)
        (:else)))
    (:else)))

(event Custom|Ranged%20Damage%20Server
  (params (Damaged%20Actor :type Actor%20Object%20Reference) (Damage :type Dmg%20Structure))
  ;[1 0 0] Damage Event
  (bind _asbpi_health_interface (Utilities|Casting|CastToBPI_HealthInterface Damaged%20Actor))
  (Default|Damage _asbpi_health_interface Damage))

(event Custom|Fire%20Effects%20Multi
  (params (Player :type BP%20Character%20Base%20Object%20Reference))
  (Networking|SwitchHasAuthority
    (:Remote
      (if (!= Player (Game|Player|GetPlayerPawn 0))
        (switch Utilities|FlowControl|Switch|SwitchonEWeaponClass (Variables|Default|GetWeapon%20Class)
          (:NewEnumerator5
            _)
          (:NewEnumerator12
            _)
          (:NewEnumerator6
            _)
          (:NewEnumerator7
            _)
          (:NewEnumerator14
            _))
        (Game|SpawnActorfromClass "/Game/Loadouts/Weapons/Ranged/Projectiles/BP_MuzzleFlash.BP_MuzzleFlash_C" (Math|Transform|MakeTransform (stale Custom|Spawn%20Projectile/Raytrace%20and%20Effects Fire%20from%20Location) "0, 0, 0" "1,1,1") "Undefined" 0 0)))))

(event Custom|Fire%20Effects%20Server
  (params (Player :type BP%20Character%20Base%20Object%20Reference))
  (CallFunction|FireEffectsMulti Player))

(event Custom|On%20Reload
  (bind _reload_animation (Variables|Default|GetReload%20Animation)
    (:then
      (Components|Animation|PlayAnimation (Variables|Default|GetLoadoutComponent%20SkeletalMesh) _reload_animation false))
    (:else)))

(event Custom|Spawn%20Projectile%20Multi
  (params (Player :type BP%20Character%20Base%20Object%20Reference) (Camera :type Scene%20Component%20Object%20Reference) (Camera%20Transform :type Transform%20%28by%20ref%29) (Projectile%20Velocity%20Modifier%20%28+/-%29 :type Float%20%28single-precision%29) (Consistent%20Inaccuracy%20Vector :type Vector) (Combustion%20Rifle%20Consistent%20Inaccuracy%20Vectors :type Array%20of%20Vectors) (Fire%20from%20Location :type Vector))
  ;[1 0.2666 0] Projectile
  (if (!= Player (Game|Player|GetPlayerPawn 0))
    (CallFunction|SpawnProjectile Player Camera Camera%20Transform Projectile%20Velocity%20Modifier%20%28+/-%29 Consistent%20Inaccuracy%20Vector Combustion%20Rifle%20Consistent%20Inaccuracy%20Vectors Fire%20from%20Location)))

(event EventBeginPlay
  (|CallParentFunction)
  (Variables|Other|SetAmmo (Variables|WeaponInformation|Projectiles|GetMax%20Ammo))
  (Variables|Default|SetADS%20Socket%20Transform (Transformation|GetSocketTransform (Variables|Default|GetLoadoutComponent%20SkeletalMesh) "ADS" "RTS_Component")))

(fn ConstructionScript
  (|CallParentFunction))

(fn Fire
  (params (Player :type BP%20Character%20Base%20Object%20Reference) (Player%20Camera :type Camera%20Component%20Object%20Reference) (Camera%20Transform :type Transform) (Projectile%20Velocity%20Modifier%20%28+/-%29 :type Float%20%28single-precision%29) (Projectile%20Spawn%20Location :type Vector))
  (CallFunction|OnFire)
  (CallFunction|SpawnProjectile/RaytraceandEffects Player Player%20Camera Camera%20Transform Projectile%20Velocity%20Modifier%20%28+/-%29 (Variables|WeaponInformation|Firing/Handling|GetShots%20per%20Click) Projectile%20Spawn%20Location))

(fn GetProjectileType
  (bind _weapon_name (Variables|Default|GetWeapon%20Name))
  (bind _returnvalue (Utilities|Select :Index _weapon_name :NewEnumerator0 "NewEnumerator4" :NewEnumerator2 "NewEnumerator4" :NewEnumerator14 "NewEnumerator4" :NewEnumerator15 "NewEnumerator4" :NewEnumerator22 "NewEnumerator4" :NewEnumerator5 "NewEnumerator4" :NewEnumerator10 "NewEnumerator4" :NewEnumerator11 "NewEnumerator4" :NewEnumerator16 "NewEnumerator4" :NewEnumerator23 "NewEnumerator4" :NewEnumerator4 "NewEnumerator4" :NewEnumerator20 "NewEnumerator4" :NewEnumerator18 "NewEnumerator4" :NewEnumerator21 "NewEnumerator4" :NewEnumerator24 "NewEnumerator4" :NewEnumerator7 "NewEnumerator4" :NewEnumerator6 "NewEnumerator4" :NewEnumerator26 "NewEnumerator4" :NewEnumerator3 "NewEnumerator4" :NewEnumerator9 "NewEnumerator4" :NewEnumerator1 "NewEnumerator4" :NewEnumerator25 "NewEnumerator4" :NewEnumerator28 "NewEnumerator4" :NewEnumerator12 "NewEnumerator4" :NewEnumerator29 "NewEnumerator4" :NewEnumerator17 "NewEnumerator4" :NewEnumerator27 "NewEnumerator4" :NewEnumerator8 "NewEnumerator6" :NewEnumerator13 "NewEnumerator4" :NewEnumerator19 "NewEnumerator4"))
  (return (select (Utilities|Enum|NotEqual(Enum) _returnvalue "NewEnumerator4") _returnvalue (Utilities|Select :Index (Variables|Default|GetWeapon%20Class) :NewEnumerator0 "NewEnumerator4" :NewEnumerator1 "NewEnumerator4" :NewEnumerator2 "NewEnumerator4" :NewEnumerator3 "NewEnumerator4" :NewEnumerator4 "NewEnumerator4" :NewEnumerator5 "NewEnumerator0" :NewEnumerator12 "NewEnumerator0" :NewEnumerator6 "NewEnumerator0" :NewEnumerator7 (Utilities|Select :Index (Variables|Default|GetWeapon%20Name) :NewEnumerator0 "NewEnumerator4" :NewEnumerator2 "NewEnumerator4" :NewEnumerator14 "NewEnumerator4" :NewEnumerator15 "NewEnumerator4" :NewEnumerator22 "NewEnumerator4" :NewEnumerator5 "NewEnumerator4" :NewEnumerator10 "NewEnumerator4" :NewEnumerator11 "NewEnumerator4" :NewEnumerator16 "NewEnumerator4" :NewEnumerator23 "NewEnumerator4" :NewEnumerator4 "NewEnumerator4" :NewEnumerator20 "NewEnumerator4" :NewEnumerator18 "NewEnumerator4" :NewEnumerator21 "NewEnumerator4" :NewEnumerator24 "NewEnumerator4" :NewEnumerator7 "NewEnumerator4" :NewEnumerator6 "NewEnumerator4" :NewEnumerator26 "NewEnumerator4" :NewEnumerator3 "NewEnumerator4" :NewEnumerator9 "NewEnumerator7" :NewEnumerator1 "NewEnumerator4" :NewEnumerator25 "NewEnumerator4" :NewEnumerator28 "NewEnumerator4" :NewEnumerator12 "NewEnumerator4" :NewEnumerator29 "NewEnumerator4" :NewEnumerator17 "NewEnumerator4" :NewEnumerator27 "NewEnumerator4" :NewEnumerator8 "NewEnumerator4" :NewEnumerator13 "NewEnumerator4" :NewEnumerator19 "NewEnumerator4") :NewEnumerator14 "NewEnumerator0" :NewEnumerator8 "NewEnumerator1" :NewEnumerator9 "NewEnumerator2" :NewEnumerator10 "NewEnumerator4" :NewEnumerator13 "NewEnumerator4"))))

(fn SetAmmo
  (params (Ammo :type Integer))
  (Variables|Other|SetAmmo Ammo)
  (Default|UpdateAmmo (Variables|/Game/Loadouts/Characters/BaseClass/BP_CharacterBase.BP_CharacterBase_C|GetHUD (.AsBP%20Character%20Base (Utilities|Casting|CastToBP_CharacterBase (Components|GetOwner))))))

(fn DecrementandUpdateAmmo
  (if (!= (Variables|WeaponInformation|Projectiles|GetMax%20Ammo) 0)
    (Variables|Other|SetAmmo (Math|Integer|Clamp(Integer) (- (Variables|Other|GetAmmo) 1) 0 100))
    (bind _hud (Variables|/Game/Loadouts/Characters/BaseClass/BP_CharacterBase.BP_CharacterBase_C|GetHUD (.AsBP%20Character%20Base (Utilities|Casting|CastToBP_CharacterBase (Components|GetOwner))))
      (:then
        (Default|UpdateAmmo _hud))
      (:else))))

(fn CalculateInaccuracyVector
  (bind _returnvalue (Components|GetOwner))
  (bind _accuracy_spread (Variables|WeaponInformation|Firing/Handling|GetAccuracy/Spread))
  (bind _asbp_character_base (Utilities|Casting|CastToBP_CharacterBase _returnvalue))
  (bind _ads__ (Variables|/Game/Loadouts/Characters/BaseClass/BP_CharacterBase.BP_CharacterBase_C|GetADS%20%25 _asbp_character_base))
  (bind _returnvalue_2 (Math|Float|Lerp 2e+04 7e+03 _ads__))
  (bind _returnvalue_3 (/ _returnvalue_2 _accuracy_spread))
  (return (Math|Vector|SelectVector (Math|Vector|MakeVector 0.0 (Math|Random|RandomFloatinRange (* -0.2 _returnvalue_3) (* 0.2 _returnvalue_3)) (Math|Random|RandomFloatinRange (* -0.1 _returnvalue_3) (* 0.1 _returnvalue_3))) "0, 0, 0" (or (Utilities|Enum|Equal(Enum) (Variables|WeaponInformation|Firing/Handling|GetFire%20Type) "NewEnumerator2") (Utilities|Enum|Equal(Enum) (Variables|Default|GetWeapon%20Name) "NewEnumerator8")))))

(fn CalculateCombustionRifleInaccuracyVectors
  (bind _output_get (LocalVariables|SetVectors (Utilities|Array|MakeArray "0, 0, 0" "0, 0, 0" "0, 0, 0" "0, 0, 0" "0, 0, 0" "0, 0, 0")))
  (for (_ _array_index) _output_get
    (Utilities|Array|SetArrayElem (LocalVariables|GetVectors) _array_index (CallFunction|CalculateInaccuracyVector)))
  (return (LocalVariables|GetVectors)))

(fn SpawnProjectile
  (params (Player :type BP%20Character%20Base%20Object%20Reference) (Camera :type Scene%20Component%20Object%20Reference) (Camera%20Transform :type Transform%20%28by%20ref%29) (Projectile%20Velocity%20Modifier%20%28+/-%29 :type Float%20%28single-precision%29) (Random%20Offset :type Vector) (Combustion%20Rifle%20Consistent%20Inaccuracy%20Vectors :type Array%20of%20Vectors) (Fire%20from%20Location :type Vector))
  (bind (_spawn_transform _spawn_transform_location _spawn_transform_rotation _spawn_transform_scale _owner_instigator _velocity _weight _projectile_type _attack_damage _knockback_level _weapon _projectile_mesh _damage_falloff_amount _time_before_damage_falloff _projectile_bounce) (|GetProjectileInfo Player Camera Camera%20Transform "0, 0, 0" "0, 0, 0" "0, 0, 0" Projectile%20Velocity%20Modifier%20%28+/-%29 Random%20Offset Fire%20from%20Location))
  (if (Utilities|Enum|NotEqual(Enum) _projectile_type "NewEnumerator4")
    (bind _returnvalue (Game|SpawnActorfromClass "/Game/Loadouts/Weapons/Ranged/Projectiles/BP_Projectile.BP_Projectile_C" (Math|Transform|MakeTransform Fire%20from%20Location "0, 0, 0" (.scale _spawn_transform)) "Undefined" _owner_instigator _velocity _weight _projectile_type _knockback_level _weapon _projectile_mesh _damage_falloff_amount _time_before_damage_falloff _projectile_bounce Combustion%20Rifle%20Consistent%20Inaccuracy%20Vectors (Utilities|Struct|MakeDmg _attack_damage "NewEnumerator2" (Pawn|GetController _owner_instigator) _weapon (Variables|Default|GetStatus%20Effects) false false false) _owner_instigator)))
  (return _returnvalue))

(fn GetAmmoInfo
  (bind _ammo (Variables|Other|GetAmmo))
  (bind _max_ammo (Variables|WeaponInformation|Projectiles|GetMax%20Ammo))
  (return _ammo _max_ammo (/ (Math|Conversions|ToFloat(Integer) _ammo) (Math|Conversions|ToFloat(Integer) _max_ammo))))

(fn Mod21
  (params (Headhunter%20Boost :type Float%20%28single-precision%29))
  (Variables|Default|SetHeadshot%20Multiplier (+ (Variables|Default|GetHeadshot%20Multiplier) Headhunter%20Boost)))

(fn Mod22
  (CallFunction|Mod21 0.3))

(fn Mod23
  (CallFunction|Mod21 0.4))