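; Revv pistol weapon whose hits cause an explosion at the point of impact.
; On any hit it runs the parent logic, then has the main game state spawn a debug-drawn area of effect that ignores line of sight.
; Each actor caught is damaged through the health interface, flagged to ignore modifiers and blocking and credited to player controller 0.
; It also supplies its own kill-feed death message.
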(event `self.On Hit Anything`
  (params (`Hit Result` :type "HitResult Structure"))
  (`parent.On Hit Anything` `Hit Result`)
  (`/Game/Loadouts/Characters/BaseClass/BP_MainGameState.Spawn AOE` (cast `/Game/Loadouts/Characters/BaseClass/BP_MainGameState` (`GameplayStatics.GetGameState`) :!pure true) (`.Location` (`GameplayStatics.BreakHitResult` `Hit Result`)) 300.0 false null (delegate `Hit by Explosion`) 1.0 (struct :`R` 1.0 :`G` 0.213405 :`A` 1.0)))

(event `Hit by Explosion`
  (params (`Hit Actor` :type "Actor Object Reference"))
  (bind _asbpi_health_interface (cast `/Game/HealthInterface/BPI_HealthInterface` `Hit Actor`))
  (`/Game/HealthInterface/BPI_HealthInterface.Damage` _asbpi_health_interface (make `/Game/HealthInterface/Dmg` 0.0 "NewEnumerator2" (`GameplayStatics.GetPlayerController` 0) self _ false false true)))

(fn `Death Message`
  (params (Killer :type "/Game/UI/In-Game/Chat/STextColor Structure") (Killed :type "/Game/UI/In-Game/Chat/STextColor Structure"))
  (returns (`Death Message` :type "Array of /Game/UI/In-Game/Chat/STextColor Structure"))
  (return (`|MakeArray` Killer (make `/Game/UI/In-Game/Chat/STextColor` " Revv" (`self.Color`)) (make `/Game/UI/In-Game/Chat/STextColor` "'d up on ") Killed)))

(fn `UserConstructionScript`
  (`parent.UserConstructionScript`))