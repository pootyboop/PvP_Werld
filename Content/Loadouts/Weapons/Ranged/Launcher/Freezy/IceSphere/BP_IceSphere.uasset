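; BP_IceSphere is a short-lived, damageable ice sphere, filed under the Freezy ranged launcher weapon.
; It destroys itself after a fixed delay from BeginPlay, or sooner once incoming damage drives its Health below zero.
; The Damage event subtracts the DamageInformation amount and prints the remaining Health to screen as debug output.
; GetHealthAsRatio is a stub that always returns zero.
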(event `self.ReceiveBeginPlay`
  (`KismetSystemLibrary.Delay` 6.0)
  (`self.K2_DestroyActor` :!label _label))

(event `/Game/HealthInterface/BPI_HealthInterface.Damage`
  (params (`Damage Information` :type "/Game/HealthInterface/Dmg Structure"))
  (bind _output_get (set `self.Health` (- (`self.Health`) `Damage Information_Damage_2_390607314C7D738086617A977C8A56C6`)))
  (`KismetSystemLibrary.PrintString` (`KismetStringLibrary.Conv_DoubleToString` _output_get))
  (if (< _output_get 0.0)
    (goto _label)))

(fn `GetHealthAsRatio`
  (returns (`Health As Ratio` :type "Float (double-precision)"))
  (return 0.0))

(fn `UserConstructionScript`)