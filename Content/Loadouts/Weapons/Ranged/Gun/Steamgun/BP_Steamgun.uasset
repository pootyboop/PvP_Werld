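; BP_Steamgun is a ranged gun weapon that spawns a steam particle effect wherever it hits and supplies its own "Steam-beamed" death message.
; Firing defers to the parent class.
; On a hit, the authority calls the multi event directly, while a remote routes through the server event, and the multi event spawns P_Steamgun at the hit location.
; An unconnected particle activation remains in the graph.
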(event `self.On Fire`
  (`parent.On Fire`))

(event `/Game/Loadouts/Weapons/BP_Weapon.On Hit Anything`
  (params (`Hit Result` :type "HitResult Structure"))
  (`/Engine/EditorBlueprintResources/ActorMacros.Switch Has Authority`
    (:`Authority`
      (`self.Steamgun Particles Multi` `Hit Result_Location`))
    (:`Remote`
      (`self.Steamgun Particles Server` `Hit Result_Location`))))

(event `Steamgun Particles Server`
  (params (Location :type "Vector Structure"))
  (`self.Steamgun Particles Multi` Location))

(event `Steamgun Particles Multi`
  (params (Location :type "Vector Structure"))
  (`NiagaraFunctionLibrary.SpawnSystemAtLocation` "/Game/Loadouts/Weapons/Ranged/Gun/Steamgun/P_Steamgun.P_Steamgun" Location))

(fn `Death Message`
  (params (Killer :type "/Game/UI/In-Game/Chat/STextColor Structure") (Killed :type "/Game/UI/In-Game/Chat/STextColor Structure"))
  (returns (`Death Message` :type "Array of /Game/UI/In-Game/Chat/STextColor Structure"))
  (return (`|MakeArray` Killer (make `/Game/UI/In-Game/Chat/STextColor` " Steam" (`self.Color`)) (make `/Game/UI/In-Game/Chat/STextColor` "-beamed ") Killed)))

(fn `UserConstructionScript`
  (`parent.UserConstructionScript`))