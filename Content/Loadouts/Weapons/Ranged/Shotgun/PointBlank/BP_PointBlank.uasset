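; BP_PointBlank is a shotgun weapon Blueprint that defines three of its mods and its "Blanked" kill message.
; Each mod sets a flag and fixes its mesh visibility; Destabilizer also raises Kick, while Funnel Cap trades damage, range and accuracy for a different fire type with burst delay.
; With Tracking Mics, MicSphere overlaps maintain a list of nearby characters other than the owner, printing their names as they arrive.
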(event `self.MicSphere.OnComponentBeginOverlap`
  (params (OverlappedComponent :type "PrimitiveComponent Object Reference") (OtherActor :type "Actor Object Reference") (OtherComp :type "PrimitiveComponent Object Reference") (OtherBodyIndex :type Integer) (bFromSweep :type Boolean) (SweepResult :type "HitResult Structure (by ref)"))
  (bind _player (`self.Use Tracking Mics` OtherActor)
    (:`true`
      (if (not (`KismetArrayLibrary.Array_Contains` (`self.Heard Players`) _player))
        (`KismetArrayLibrary.Array_Add` (`self.Heard Players`) _player)
        (`KismetSystemLibrary.PrintString` (`KismetStringLibrary.Concat_StrStr` (`KismetSystemLibrary.GetDisplayName` _player) " is nearby!"))))))

(event `self.MicSphere.OnComponentEndOverlap`
  (params (OverlappedComponent :type "PrimitiveComponent Object Reference") (OtherActor :type "Actor Object Reference") (OtherComp :type "PrimitiveComponent Object Reference") (OtherBodyIndex :type Integer))
  (bind _player (`self.Use Tracking Mics` OtherActor)
    (:`true`
      (`KismetArrayLibrary.Array_RemoveItem` (`self.Heard Players`) _player))))

(fn `Death Message`
  (params (Killer :type "/Game/UI/In-Game/Chat/STextColor Structure") (Killed :type "/Game/UI/In-Game/Chat/STextColor Structure"))
  (returns (`Death Message` :type "Array of /Game/UI/In-Game/Chat/STextColor Structure"))
  (return (`|MakeArray` Killer (make `/Game/UI/In-Game/Chat/STextColor` " Blanked " (`self.Color`)) Killed)))

(fn `Mod_6`
  (set `self.hasTrackingMics` true)
  (`self.Fix Mod Mesh Visibility` (`self.Tracking Mics`)))

(fn `Mod_7`
  (set `self.hasDestabilizer` true)
  (`self.Fix Mod Mesh Visibility` (`self.Destabilizer`))
  (set `self.Kick` (+ (`self.Kick`) 5.0)))

(fn `Mod_8`
  (set `self.hasFunnelCap` true)
  (`self.Fix Mod Mesh Visibility` (`self.Funnel Cap`))
  (set `self.Attack Damage` (- (`self.Attack Damage`) 2.0))
  (set `self.Attack Range` (- (`self.Attack Range`) 1.0))
  (set `self.Fire Type` "NewEnumerator3")
  (set `self.Burst/Blast Delay` 0.1)
  (set `self.Accuracy/Spread` (+ (`self.Accuracy/Spread`) 2.0)))

(fn `UserConstructionScript`
  (`self.Add Meshes` (`|MakeArray` (`self.Destabilizer`) (`self.Funnel Cap`) (`self.Tracking Mics`) :!type "PrimitiveComponent Object Reference"))
  (`parent.UserConstructionScript`))