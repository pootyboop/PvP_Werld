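; Shared projectile for ranged weapons, configured by type as bullet, arrow, bolt, ice sphere or combustion shot.
; Damage scales with the shooter's Ranged attack, then decays on authority after a delay as gravity increases.
; Combustion shots split into bullets after a timer.
; Hits apply authority-side damage, headshot flags and launch knockback to health-interface actors; other impacts bounce, destroy, disarm or spawn an ice sphere by type.
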(event `self.ReceiveBeginPlay`
  (bind _damage_info_damage (break `/Game/HealthInterface/Dmg` (`self.Damage Info`)))
  (bind (_damage_info_damage_2 _damage_info_damagetype _damage_info_instigator _damage_info_literaldamagedealer _damage_info_statuseffects _damage_info_isheadshot _damage_info_isspecialdamage) (break `/Game/HealthInterface/Dmg` (`self.Damage Info`)))
  (bind (_attack_melee _attack_ranged) (break `/Game/Loadouts/Characters/BaseClass/DamageTypeModifier` (`/Game/Loadouts/Characters/BaseClass/BP_CharacterBase.Attack` (cast `/Game/Loadouts/Characters/BaseClass/BP_CharacterBase` (`self.Instigator`) :!pure true))))
  (set `MovementComponent.Velocity` (`self.Velocity`) (`self.ProjectileMovement`))
  (set `ProjectileMovementComponent.ProjectileGravityScale` (`self.Weight`) (`self.ProjectileMovement`))
  (set `self.Damage` (* _damage_info_damage (/ _attack_ranged 5.0)))
  (set `ProjectileMovementComponent.bShouldBounce` (`self.Bounces`) (`self.ProjectileMovement`))
  (`self.SetOwner` (`self.GetInstigator`))
  (`PrimitiveComponent.IgnoreActorWhenMoving` (`self.Sphere`) (`self.GetOwner`) true)
  (`PrimitiveComponent.IgnoreActorWhenMoving` (`self.Sphere`) (`self.Weapon`) true)
  (`|ExecutionSequence`
    (:`then_0`
      (bind _outactors (`GameplayStatics.GetAllActorsOfClass` "/Game/Loadouts/Characters/BaseClass/BP_CharacterBase.BP_CharacterBase_C"))
      (for _array_element _outactors
        (`PrimitiveComponent.IgnoreComponentWhenMoving` (`Character.CapsuleComponent` _array_element) (`Character.CapsuleComponent` _array_element) true)))
    (:`then_1`
      (bind _outactors_2 (`GameplayStatics.GetAllActorsOfClass` "BP_Projectile_C"))
      (for _array_element_2 _outactors_2
        (if (== (`self.GetOwner`) (`self.GetOwner` _array_element_2))
          (`PrimitiveComponent.IgnoreActorWhenMoving` (`self.Sphere`) _array_element_2 true)
          (`self.Ignore Actor` (cast `/Game/Loadouts/Weapons/Ranged/Projectiles/BP_Projectile` _array_element_2 :!pure true) self)))
      (`StaticMeshComponent.SetStaticMesh` (`self.StaticMesh`) (`self.New Static Mesh`))
      (if (`|EnumEquality` (`self.Type`) "NewEnumerator6") :!label _label
        ;[1 1 1] Combustion Rifle
        (`KismetSystemLibrary.RetriggerableDelay` (`/Game/Loadouts/Weapons/Ranged/Shotgun/CombustionRifle/BP_CombustionRifle.Time before Projectile Combustion` (cast `/Game/Loadouts/Weapons/Ranged/Shotgun/CombustionRifle/BP_CombustionRifle` (`self.Weapon`) :!pure true)))
        (for _array_element_3 (`self.Consistent Inaccuracy Vectors`)
          (`|SpawnActorFromClass` :`Class` "BP_Projectile_C" :`SpawnTransform` (`SceneComponent.K2_GetComponentToWorld` (`self.StaticMesh`)) :`CollisionHandlingOverride` "Undefined" :`TransformScaleMethod` "OverrideRootScale" :`Velocity` (+ (* (`self.Velocity`) 2) _array_element_3) :`Weight` 0.0 :`Type` "NewEnumerator0" :`Knockback` (`self.Knockback`) :`Weapon` (`self.Weapon`) :`New Static Mesh` "/Game/Loadouts/Weapons/Ranged/Projectiles/bullet_default.bullet_default" :`Time before Damage Falloff` 0.2 :`Damage Info` (make `/Game/HealthInterface/Dmg` (`self.Damage`) _damage_info_damagetype _damage_info_instigator _damage_info_literaldamagedealer _damage_info_statuseffects false _damage_info_isspecialdamage) :`Instigator` (`self.Instigator`)))
        (`self.K2_DestroyActor`)
        (else
          (`KismetSystemLibrary.RetriggerableDelay` (`self.Time before Damage Falloff`))
          (set `self.Falloff Active` true))))))

(event `self.ReceiveTick`
  (params (DeltaSeconds :type "Float (single-precision)"))
  (bind _projectilemovement (`self.ProjectileMovement`))
  (if (`self.Falloff Active`)
    (set `ProjectileMovementComponent.ProjectileGravityScale` (+ (`ProjectileMovementComponent.ProjectileGravityScale` _projectilemovement) 2.0) _projectilemovement)
    (`/Engine/EditorBlueprintResources/ActorMacros.Switch Has Authority`
      (:`Authority`
        (set `self.Damage` (`KismetMathLibrary.FClamp` (- (`self.Damage`) (/ (`self.Damage Falloff Amount`) 1500.0)) 0.5 100.0))))))

(event `self.ReceiveHit`
  (params (MyComp :type "PrimitiveComponent Object Reference") (Other :type "Actor Object Reference") (OtherComp :type "PrimitiveComponent Object Reference") (bSelfMoved :type Boolean) (HitLocation :type "Vector Structure") (HitNormal :type "Vector Structure") (NormalImpulse :type "Vector Structure") (Hit :type "HitResult Structure (by ref)"))
  (bind (_bblockinghit _binitialoverlap _time _distance _location _impactpoint _normal _impactnormal _physmat _hitactor _hitcomponent _hitbonename) (`GameplayStatics.BreakHitResult` Hit))
  (bind _returnvalue (`self.GetInstigator`))
  (bind (_returnvalue_location _returnvalue_rotation) (`KismetMathLibrary.BreakTransform` (`SceneComponent.K2_GetComponentToWorld` (`self.Sphere`))))
  (bind (_asbpi_health_interface _bsuccess) (cast `/Game/HealthInterface/BPI_HealthInterface` _hitactor :!pure true))
  (if (!= Other (`self.GetOwner` (`self.Weapon`)))
    (`/Game/Loadouts/Weapons/BP_Weapon.On Hit Anything` (`self.Weapon`) Hit)
    (if (`|EnumEquality` (`self.Type`) "NewEnumerator7")
      (if (`self.Bounces`) :!label _label_2
        (set `self.Bounced` true)
        (goto _label)
        (else
          (switch `/Game/Loadouts/Weapons/Ranged/Projectiles/EProjectileType` (`self.Type`)
            (:`NewEnumerator0`
              (`self.K2_DestroyActor` :!label _label_3))
            (:`NewEnumerator1`
              (set `self.Falloff Active` false :!label _label_4)
              (set `self.Damage` 0.0))
            (:`NewEnumerator2`
              (goto _label_4))
            (:`NewEnumerator7`
              (`|SpawnActorFromClass` "/Game/Loadouts/Weapons/Ranged/Launcher/Freezy/IceSphere/BP_IceSphere.BP_IceSphere_C" (`KismetMathLibrary.MakeTransform` _returnvalue_location _returnvalue_rotation) "Undefined" "OverrideRootScale" _returnvalue _returnvalue)
              (`self.K2_DestroyActor`))
            (:`NewEnumerator6`
              (goto _label_3)))))
      (elif _bsuccess
        (`/Engine/EditorBlueprintResources/ActorMacros.Switch Has Authority`
          (:`Authority`
            (bind _structout (setmembers `/Game/HealthInterface/Dmg` :`StructRef` (`self.Damage Info`) :`Damage` (* 2 (`self.Damage`)) :`Is Headshot` (`/Game/BPFunctionLibrary.Is Bone Headshot` _hitbonename)))
            (`/Game/HealthInterface/BPI_HealthInterface.Damage` _asbpi_health_interface _structout)
            (`/Game/Loadouts/Weapons/BP_Weapon.Hit Opponent` (`self.Weapon`) (cast `/Game/Loadouts/Characters/BaseClass/BP_CharacterBase` _asbpi_health_interface :!pure true) _structout 0)
            (bind _asbp_character_base (cast `/Game/Loadouts/Characters/BaseClass/BP_CharacterBase` _hitactor)
              (:`then`
                (`Character.LaunchCharacter` _asbp_character_base (* (`SceneComponent.GetForwardVector` (`/Game/Loadouts/Characters/BaseClass/BP_CharacterBase.Camera` (cast `/Game/Loadouts/Characters/BaseClass/BP_CharacterBase` (`self.GetInstigator`) :!pure true))) (* 1000 (`/Game/Loadouts/Weapons/BP_Weapon.Attack Punch` (`self.Weapon`)))) false false))
              (:`CastFailed`
                _)))
          (:`Remote`
            _))
        (`self.K2_DestroyActor`)
        (else
          (goto _label_2))))))

(fn `Ignore Actor`
  (params (Actor :type "Actor Object Reference"))
  (`PrimitiveComponent.IgnoreActorWhenMoving` (`self.Sphere`) Actor true))

(fn `UserConstructionScript`)