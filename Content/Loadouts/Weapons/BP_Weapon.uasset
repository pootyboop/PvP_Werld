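; Base weapon actor that players pick up, equip and drop, with a slot-costed mod system and empty combat hooks.
; A weapon state switches collision and physics for Dropped, Equipped and Menu, with an optional despawn timer for dropped weapons.
; Equipped mods run by building "Mod_<ID>" function names for short timers, changing stats or starting periodic healing scaled by free slots.
; Materials are applied across all registered weapon and mod meshes.
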(event `self.ReceiveTick`
  (params (DeltaSeconds :type "Float (single-precision)"))
  (`parent.ReceiveTick` DeltaSeconds))

(event `Plain Jane Timer`
  (`KismetSystemLibrary.K2_SetTimerDelegate` (delegate `Plain Jane Heal`) 2.0 true))

(event `Plain Jane Heal`
  (bind _returnvalue (`self.GetOwner`))
  (`/Engine/EditorBlueprintResources/StandardMacros.IsValid` _returnvalue
    (:`Is Valid`
      (bind _asbp_character_base (cast `/Game/Loadouts/Characters/BaseClass/BP_CharacterBase` _returnvalue))
      (if (== (`/Game/Loadouts/Characters/BaseClass/BP_CharacterBase.Get Equipped Weapon` _asbp_character_base) self)
        (message `/Game/HealthInterface/BPI_HealthInterface.Heal` (`self.GetOwner`) (* (`self.Free Mod Slots`) 0.5))))))

(event `Setup Mods Multi`
  (params (ModLevelsMultiProof :type "/Game/Loadouts/Weapons/Mods/ModLevels Structure"))
  ;[1 1 1] Spawn
  (bind _asbp_character_base (cast `/Game/Loadouts/Characters/BaseClass/BP_CharacterBase` (`self.GetOwner`)))
  (if (`Pawn.IsLocallyControlled` _asbp_character_base)
    (`KismetSystemLibrary.PrintString` "verify" true true (struct :`A` 1.0))
    (for (_array_element _array_index) (`.Equipped_11_5E7168F145FFCB405FD71A8D5073BBBC` (break `/Game/Loadouts/Weapons/Mods/ModLevels` ModLevelsMultiProof))
      (if _array_element
        (`KismetSystemLibrary.PrintString` (`KismetStringLibrary.Conv_IntToString` _array_index) true true (struct :`R` 1.0 :`G` 0.148209 :`A` 1.0))))
    (`self.Process Mods` ModLevelsMultiProof)))

(event `self.ReceiveBeginPlay`
  ;[1 1 1] Spawn
  (`parent.ReceiveBeginPlay`)
  (`self.SetWeaponState` (`self.Weapon State`) false))

(event `/Game/InteractionInterface/InteractionInterface.OnInteracted`
  (params (Player :type "/Game/Loadouts/Characters/BaseClass/BP_CharacterBase Object Reference"))
  (`parent.OnInteracted` Player)
  (`self.Pick Up Weapon` Player))

(event `Pick Up Weapon`
  (params (Player :type "/Game/Loadouts/Characters/BaseClass/BP_CharacterBase Object Reference"))
  ;[1 1 1] Pick up
  (`self.Destroy Interaction Widget`)
  (`/Game/Loadouts/Characters/BaseClass/BP_CharacterBase.Pick Up Weapon (new)` Player self)
  (`/Game/Loadouts/Characters/BaseClass/BP_CharacterBase.Set Weapon State (on character)` Player "NewEnumerator1" self))

(event `Despawn Timer`
  (`KismetSystemLibrary.RetriggerableDelay` 15.0)
  (switch `/Game/Loadouts/Weapons/EWeaponState` (`self.Weapon State`)
    (:`NewEnumerator0`
      (`self.K2_DestroyActor`))))

(event `Special Pressed`)

(event `Special Released`)

(event `Hit Opponent`
  (params (Player :type "/Game/Loadouts/Characters/BaseClass/BP_CharacterBase Object Reference") (Damage :type "/Game/HealthInterface/Dmg Structure") (`Combo #` :type Integer)))

(event `On Hit Anything`
  (params (`Hit Result` :type "HitResult Structure")))

(event `On Kill`
  (params (Damage :type "/Game/HealthInterface/Dmg Structure")))

(event `On Owning Player Damaged`
  (params (Damage :type "/Game/HealthInterface/Dmg Structure")))

(event `Setup Multi`
  (`KismetSystemLibrary.Delay` 0.1)
  (`self.Process Mods` (`self.Mod Levels`))
  (`self.Update Materials`))

(fn `Add Material`
  (params (Material :type "MaterialInstance Object Reference") (Slot :type Integer))
  (for _array_element (`self.Weapon Meshes`)
    (`PrimitiveComponent.SetMaterial` _array_element Slot Material)))

(fn `Add Meshes`
  (params (SourceArray :type "Array of PrimitiveComponent Object Reference (by ref)"))
  (`KismetArrayLibrary.Array_Append` (`self.Weapon Meshes`) SourceArray))

(fn `Calculate Basic Flat Attack Damage`
  (returns (`Final Flat Damage` :type "Float (double-precision)"))
  (return (`self.Attack Damage`)))

(fn `Death Message`
  (params (Killer :type "/Game/UI/In-Game/Chat/STextColor Structure") (Killed :type "/Game/UI/In-Game/Chat/STextColor Structure"))
  (returns (`Death Message` :type "Array of /Game/UI/In-Game/Chat/STextColor Structure"))
  (locals (`Weapon Message 1` :type Text :default "NSLOCTEXT(\"\", \"8C8FD10A4AED55930A18E8BE5D9A3DFB\", \" used \")") (`Weapon Message 2` :type Text :default "NSLOCTEXT(\"\", \"552D392643163991BCE705B026D30F87\", \" to kill \")"))
  (return (`|MakeArray` Killer (make `/Game/UI/In-Game/Chat/STextColor` (`local.Weapon Message 1`)) (make `/Game/UI/In-Game/Chat/STextColor` (`KismetTextLibrary.Conv_StringToText` (`|GetEnumeratorNameAsString` (`self.Weapon Name`))) (`self.Color`)) (make `/Game/UI/In-Game/Chat/STextColor` (`local.Weapon Message 2`)) Killed)))

(fn `Drop`
  (params (Player :type "/Game/Loadouts/Characters/BaseClass/BP_CharacterBase Object Reference"))
  (`/Game/Loadouts/Characters/BaseClass/BP_CharacterBase.Set Weapon State (on character)` Player "NewEnumerator0" self)
  (`/Game/Loadouts/Characters/BaseClass/BP_CharacterBase.Destroy 1st Person Weapon` Player))

(fn `Fix Mod Mesh Visibility`
  (params (Mesh :type "PrimitiveComponent Object Reference"))
  (bind _returnvalue (`self.GetOwner`))
  (bind _mesh (`local.Mesh`))
  (`SceneComponent.SetHiddenInGame` Mesh false false)
  (`KismetArrayLibrary.Array_AddUnique` (`self.Weapon Meshes`) Mesh)
  (`self.Update Materials`)
  (`/Engine/EditorBlueprintResources/StandardMacros.IsValid` _returnvalue
    (:`Is Valid`
      (bind _is_1st_person_weapon (`/Game/Loadouts/Characters/BaseClass/BP_CharacterBase.Is 1st Person Weapon` (cast `/Game/Loadouts/Characters/BaseClass/BP_CharacterBase` _returnvalue :!pure true) self))
      (if _is_1st_person_weapon
        (`PrimitiveComponent.SetOnlyOwnerSee` _mesh true)
        (else
          (`PrimitiveComponent.SetOwnerNoSee` _mesh true))))))

(fn `GetInteractionText`
  (returns (Text :type Text))
  (return (`KismetTextLibrary.Conv_StringToText` (`|GetEnumeratorNameAsString` (`self.Weapon Name`)))))

(fn `GetInteractionTextAttach`
  (returns (AttachComponent :type "SceneComponent Object Reference"))
  (return (`self.LoadoutComponent SkeletalMesh`)))

(fn `Has Mod by ID`
  (params (`Mod ID` :type Integer))
  (returns (Output :type Boolean))
  (bind _mod_levels_equipped (break `/Game/Loadouts/Weapons/Mods/ModLevels` (`self.Mod Levels`)))
  (return (`|GetArrayItem` _mod_levels_equipped (- `Mod ID` 1))))

(fn `Mod_0`)

(fn `Mod_1`
  (set `self.Attack Damage` (+ (`self.Attack Damage`) 2.0)))

(fn `Mod_10`)

(fn `Mod_11`)

(fn `Mod_12`)

(fn `Mod_13`
  (`self.Update Free Mod Slots`)
  (if (!= (`self.Free Mod Slots`) 0)
    (`self.Plain Jane Timer`)))

(fn `Mod_14`)

(fn `Mod_15`
  (`self.Mod_1`))

(fn `Mod_16`
  (`self.Mod_1`))

(fn `Mod_17`
  (`self.Mod_2`))

(fn `Mod_18`
  (`self.Mod_2`))

(fn `Mod_19`
  (`self.Mod_3`))

(fn `Mod_2`
  (set `self.Attack Speed` (+ (`self.Attack Speed`) 2.0)))

(fn `Mod_20`
  (`self.Mod_3`)
  (`self.Mod_3`))

(fn `Mod_21`
  (params (`Headhunter Boost` :type "Float (double-precision)" :default 0.3)))

(fn `Mod_22`)

(fn `Mod_23`)

(fn `Mod_3`
  (set `self.Attack Range` (+ (`self.Attack Range`) 2.0)))

(fn `Mod_4`
  (set `self.Attack Punch` (+ (`self.Attack Punch`) 1.0)))

(fn `Mod_5`
  (set `self.Neutralizing` true))

(fn `Mod_6`)

(fn `Mod_7`)

(fn `Mod_8`)

(fn `Mod_9`)

(fn `OnRep_IsInit`
  (`/Game/Loadouts/Characters/BaseClass/BP_CharacterBase.Loadout Weapon Delay` (cast `/Game/Loadouts/Characters/BaseClass/BP_CharacterBase` (`self.GetOwner`) :!pure true) self))

(fn `Process Mods`
  (params (ModLevelsMultiProof :type "/Game/Loadouts/Weapons/Mods/ModLevels Structure"))
  (for (_array_element _array_index) (`.Equipped_11_5E7168F145FFCB405FD71A8D5073BBBC` (break `/Game/Loadouts/Weapons/Mods/ModLevels` ModLevelsMultiProof))
    (if _array_element
      (`self.Set Up Mod` (+ _array_index 1)))))

(fn `Set Up Mod`
  (params (`Mod ID` :type Integer :default 1))
  (`KismetSystemLibrary.K2_SetTimer` self (`KismetStringLibrary.Concat_StrStr` "Mod_" (`KismetStringLibrary.Conv_IntToString` `Mod ID`)) 0.0001))

(fn `SetWeaponState`
  (params (`New Weapon State` :type "/Game/Loadouts/Weapons/EWeaponState Enum" :default "NewEnumerator0") (startDespawnTimer :type Boolean :default true))
  (bind _loadoutcomponent_skeletalmesh (`self.LoadoutComponent SkeletalMesh`))
  (bind _sphere (`self.Sphere`))
  (bind _output_get (set `self.Weapon State` `New Weapon State`))
  (switch `/Game/Loadouts/Weapons/EWeaponState` _output_get
    (:`NewEnumerator0`
      (`PrimitiveComponent.SetCollisionProfileName` _sphere "OverlapAllDynamic" true)
      (`PrimitiveComponent.SetSimulatePhysics` _loadoutcomponent_skeletalmesh true)
      (`PrimitiveComponent.SetCollisionProfileName` _loadoutcomponent_skeletalmesh "DroppedWeapon" true)
      (if (`local.startDespawnTimer`)
        (`self.Despawn Timer`)))
    (:`NewEnumerator1`
      (`PrimitiveComponent.SetCollisionProfileName` _sphere "NoCollision" true)
      (`PrimitiveComponent.SetSimulatePhysics` _loadoutcomponent_skeletalmesh false)
      (`PrimitiveComponent.SetCollisionProfileName` _loadoutcomponent_skeletalmesh "NoCollision" true)
      (`SceneComponent.ResetRelativeTransform` _loadoutcomponent_skeletalmesh))
    (:`NewEnumerator2`
      (`PrimitiveComponent.SetCollisionProfileName` _sphere "NoCollision" true)
      (`PrimitiveComponent.SetSimulatePhysics` _loadoutcomponent_skeletalmesh true)
      (`PrimitiveComponent.SetCollisionProfileName` _loadoutcomponent_skeletalmesh "NoCollision" true)
      (`SceneComponent.ResetRelativeTransform` _loadoutcomponent_skeletalmesh)
      (`PrimitiveComponent.SetCollisionEnabled` _loadoutcomponent_skeletalmesh "NoCollision"))))

(fn `Update Free Mod Slots`
  (bind _mod_levels_equipped (break `/Game/Loadouts/Weapons/Mods/ModLevels` (`self.Mod Levels`)))
  (set `self.Free Mod Slots` (`self.Max Mod Capacity`))
  (for (_array_element _array_index) _mod_levels_equipped
    (if _array_element
      (set `self.Free Mod Slots` (- (`self.Free Mod Slots`) (`.Cost_43_38B6459A4D80DA76F5D5BE899C4057FE` (break `/Game/Loadouts/Weapons/Mods/Mod` (`/Game/BPFunctionLibrary.Get Mod Info` (+ _array_index 1)))))))))

(fn `Update Materials`
  (for (_array_element _array_index) (`self.Materials`)
    (`/Engine/EditorBlueprintResources/StandardMacros.IsValid` _array_element
      (:`Is Valid`
        (for _array_element_2 (`self.Weapon Meshes`)
          (`PrimitiveComponent.SetMaterial` _array_element_2 _array_index _array_element))))))

(fn `UserConstructionScript`
  (`parent.UserConstructionScript`)
  (`KismetArrayLibrary.Array_AddUnique` (`self.Weapon Meshes`) (`self.LoadoutComponent SkeletalMesh`))
  (`self.Update Materials`)
  (set `self.Name` (`KismetTextLibrary.Conv_StringToText` (`|GetEnumeratorNameAsString` (`self.Weapon Name`))))
  (`self.Setup Multi`))