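; Vaulter spear, a melee weapon whose special launches its owner upward and along the camera's forward direction, boosting attack damage.
; The vault runs locally and through a server event to mask lag, with particles multicast to non-local players.
; A looping timer polls for landing, then restores damage and re-arms the vault after a delay, near-instant for wall-jump resets.
; It also supplies a custom "Vaulted over" kill message.
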(event `self.ReceiveBeginPlay`
  (`parent.ReceiveBeginPlay`)
  (set `self.Default Attack Damage` (`self.Attack Damage`)))

(event `self.Special Pressed`
  (`self.Try to Vault`))

(event `Try to Vault`
  (bind (_returnvalue_x _returnvalue_y) (`KismetMathLibrary.BreakVector` (* (`SceneComponent.GetForwardVector` (`/Game/Loadouts/Characters/BaseClass/BP_CharacterBase.Camera` (`self.Player`))) (`self.Horizontal Vault Force`))))
  (if (not (`self.isVaulting`))
    (bind _asbp_character_base (cast `/Game/Loadouts/Characters/BaseClass/BP_CharacterBase` (`self.GetOwner`)))
    (bind _output_get (set `self.Player` _asbp_character_base))
    (if (`/Game/Loadouts/Characters/BaseClass/BP_CharacterBase.Can Vault` _output_get)
      (set `self.isVaulting` true)
      (`self.Vault Event` (`KismetMathLibrary.MakeVector` _returnvalue_x _returnvalue_y (`self.Vertical Vault Force`))) ; Runs Vault on client before server in case of lag
      (`/Game/Loadouts/Characters/BaseClass/BP_CharacterBase.Vault Anim` (cast `/Game/Loadouts/Characters/BaseClass/BP_CharacterBase` (`self.GetOwner`) :!pure true))
      (set `self.Attack Damage` (+ (`self.Default Attack Damage`) (`self.Vault Attack Boost`)))
      (`PlayerCameraManager.StartCameraShake` :`self` (`GameplayStatics.GetPlayerCameraManager` 0) :`ShakeClass` "/Game/VisualEffects/CameraShake/BoostCameraShake.BoostCameraShake_C" :`Scale` (/ (+ (`self.Vertical Vault Force`) (`self.Horizontal Vault Force`)) 1100.0))
      (bind _returnvalue (`KismetSystemLibrary.K2_SetTimerDelegate` (delegate `Check for Vault Landing`) 0.1 true))
      (set `self.Vaulter In Air` _returnvalue))))

(event `Check for Vault Landing`
  (bind _player (`self.Player`)
    (:`then`
      (if (`NavMovementComponent.IsMovingOnGround` (`Pawn.GetMovementComponent` _player))
        (`self.Vaulter Reset` false)))
    (:`else`)))

(event `Vaulter Reset`
  (params (Walljump :type Boolean))
  (`KismetSystemLibrary.K2_ClearAndInvalidateTimerHandle` (`self.Vaulter In Air`))
  (`KismetSystemLibrary.K2_SetTimerDelegate` (delegate `Vaulter Reset (timer)`) (`KismetMathLibrary.SelectFloat` 0.001 1.0 Walljump)))

(event `Vault Event`
  (params (Velocity :type "Vector Structure"))
  (bind _player (`self.Player`))
  (`self.Vault Server` _player Velocity)
  (`self.Vault` _player Velocity)
  (`AddComponent|NODE_AddNiagaraComponent-0` :`self` _player))

(event `Vaulter Reset (timer)`
  (set `self.isVaulting` false)
  (set `self.Attack Damage` (`self.Default Attack Damage`))
  (`KismetSystemLibrary.PrintString` "vault ready!"))

(event `Vault Server`
  (params (Player :type "/Game/Loadouts/Characters/BaseClass/BP_CharacterBase Object Reference") (Velocity :type "Vector Structure"))
  (`self.Vault` Player Velocity)
  (`self.Vault Particles Multi` Player))

(event `Vault Particles Multi`
  (params (Player :type "/Game/Loadouts/Characters/BaseClass/BP_CharacterBase Object Reference"))
  (if (not (`Pawn.IsLocallyControlled` Player))
    (`AddComponent|NODE_AddNiagaraComponent-1` :`self` Player)))

(fn `Death Message`
  (params (Killer :type "/Game/UI/In-Game/Chat/STextColor Structure") (Killed :type "/Game/UI/In-Game/Chat/STextColor Structure"))
  (returns (`Death Message` :type "Array of /Game/UI/In-Game/Chat/STextColor Structure"))
  (return (`|MakeArray` Killer (make `/Game/UI/In-Game/Chat/STextColor` " Vaulted " (`self.Color`)) (make `/Game/UI/In-Game/Chat/STextColor` "over ") Killed)))

(fn `UserConstructionScript`
  (`parent.UserConstructionScript`))

(fn `Vault`
  (params (Player :type "Character Object Reference") (LaunchVelocity :type "Vector Structure"))
  (`Character.LaunchCharacter` Player LaunchVelocity false true))