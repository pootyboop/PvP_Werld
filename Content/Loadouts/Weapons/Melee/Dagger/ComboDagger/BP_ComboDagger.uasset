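; Combo dagger melee weapon that gains attack damage as its wielder keeps hitting opponents.
; Each hit restarts a five-second timer; below the level cap, a combo count of three resets the count, raises the combo level and adds damage.
; When the timer expires, EndCombo removes the bonus damage and clears level and count.
; It also supplies a combo-themed death message and prints level changes as debug text.
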(event `self.Hit Opponent`
  (params (Player :type "/Game/Loadouts/Characters/BaseClass/BP_CharacterBase Object Reference") (Damage :type "/Game/HealthInterface/Dmg Structure") (`Combo #` :type Integer))
  (`KismetSystemLibrary.K2_ClearAndInvalidateTimerHandle` (`self.Combo Dagger Timer`))
  (bind _returnvalue (`KismetSystemLibrary.K2_SetTimerDelegate` (delegate `End Combo`) 5.0))
  (set `self.Combo Dagger Timer` _returnvalue)
  (if (< (`self.Combo Lvl`) (`self.Max Combo Lvl`))
    (bind _output_get (set `self.Combo #` `Combo #`))
    (if (== _output_get 3)
      (set `self.Combo #` 0)
      (`/Engine/EditorBlueprintResources/StandardMacros.IncrementInt` (`self.Combo Lvl`)
        (:`  `
          (set `self.Attack Damage` (+ (`self.Attack Damage`) 3.0))
          (`KismetSystemLibrary.PrintString` (`KismetStringLibrary.Concat_StrStr` "Combo Lvl " (`KismetStringLibrary.Conv_IntToString` (`self.Combo Lvl`))) :!label _label))))))

(event `End Combo`
  (`KismetSystemLibrary.K2_ClearAndInvalidateTimerHandle` (`self.Combo Dagger Timer`))
  (set `self.Attack Damage` (- (`self.Attack Damage`) (`KismetMathLibrary.Conv_IntToDouble` (* (`self.Combo Lvl`) 3))))
  (set `self.Combo Lvl` 0)
  (set `self.Combo #` 0)
  (goto _label))

(fn `Death Message`
  (params (Killer :type "/Game/UI/In-Game/Chat/STextColor Structure") (Killed :type "/Game/UI/In-Game/Chat/STextColor Structure"))
  (returns (`Death Message` :type "Array of /Game/UI/In-Game/Chat/STextColor Structure"))
  (return (`|MakeArray` Killer (make `/Game/UI/In-Game/Chat/STextColor` " dropped a ") (make `/Game/UI/In-Game/Chat/STextColor` "Combo" (`self.Color`)) (make `/Game/UI/In-Game/Chat/STextColor` " on ") Killed)))

(fn `UserConstructionScript`
  (`parent.UserConstructionScript`))