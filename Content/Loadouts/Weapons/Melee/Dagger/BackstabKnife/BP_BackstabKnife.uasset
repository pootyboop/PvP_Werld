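; Backstab knife melee weapon that deals special backstab damage when striking an opponent from behind.
; On hit, it compares victim and owner forward vectors by dot product against a precision threshold, applying damage only when they align.
; A backstab shows W_Backstab on player controller 0, plus a victim variant if that controller's pawn was hit.
; It also supplies a knife-specific death message.
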(event `/Game/Loadouts/Weapons/BP_Weapon.Hit Opponent`
  (params (Player :type "/Game/Loadouts/Characters/BaseClass/BP_CharacterBase Object Reference") (Damage :type "/Game/HealthInterface/Dmg Structure") (`Combo #` :type Integer))
  (if (> (`KismetMathLibrary.Dot_VectorVector` (`self.GetActorForwardVector` Player) (`self.GetActorForwardVector` (`self.GetOwner`))) (`self.Backstab Precision Requirement`))
    (bind _structout (setmembers `/Game/HealthInterface/Dmg` :`StructRef` Damage :`Damage` (`self.Backstab Damage`) :`Is Special Damage` true))
    (`/Game/Loadouts/Characters/BaseClass/BP_CharacterBase.Damage` Player _structout)
    (`self.Backstabber`)
    (`self.Backstabbed` Player)))

(event `Backstabber`
  (bind _returnvalue (`|CreateWidget` "/Game/UI/In-Game/Weapon/W_Backstab.W_Backstab_C" (`GameplayStatics.GetPlayerController` 0)))
  (`/Engine/EditorBlueprintResources/StandardMacros.IsValid` _returnvalue
    (:`Is Valid`
      (`UserWidget.AddToViewport` _returnvalue 0))))

(event `Backstabbed`
  (params (Player :type "/Game/Loadouts/Characters/BaseClass/BP_CharacterBase Object Reference"))
  (if (== Player (`Controller.K2_GetPawn` (`GameplayStatics.GetPlayerController` 0)))
    (bind _returnvalue (`|CreateWidget` "/Game/UI/In-Game/Weapon/W_Backstab.W_Backstab_C" (`GameplayStatics.GetPlayerController` 0) true))
    (`/Engine/EditorBlueprintResources/StandardMacros.IsValid` _returnvalue
      (:`Is Valid`
        (`UserWidget.AddToViewport` _returnvalue 0)))))

(fn `Death Message`
  (params (Killer :type "/Game/UI/In-Game/Chat/STextColor Structure") (Killed :type "/Game/UI/In-Game/Chat/STextColor Structure"))
  (returns (`Death Message` :type "Array of /Game/UI/In-Game/Chat/STextColor Structure"))
  (return (`|MakeArray` Killer (make `/Game/UI/In-Game/Chat/STextColor` " took a ") (make `/Game/UI/In-Game/Chat/STextColor` "Knife" (`self.Color`)) (make `/Game/UI/In-Game/Chat/STextColor` " to ") Killed)))

(fn `UserConstructionScript`
  (`parent.UserConstructionScript`))