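; Portal sword melee weapon whose special, usable only while the player is on the ground, spawns a portal at the player's position.
; Spawns alternate between Entry and Exit types, with a FlipFlop storing them in two slots.
; Each spawn destroys that slot's old portal and inherits its paired-portal reference.
; It also supplies a portal-themed death message; blade material swap logic is present but unconnected.
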(event `/Game/Loadouts/Weapons/BP_Weapon.Special Pressed`
  (if (`NavMovementComponent.IsMovingOnGround` (`Pawn.GetMovementComponent` (`GameplayStatics.GetPlayerPawn` 0)))
    (`self.Create Portal Sword Portal`)))

(event `Create Portal Sword Portal`
  (bind _returnvalue (`GameplayStatics.GetPlayerPawn` 0))
  (bind _returnvalue_2 (`|SpawnActorFromClass` "/Game/Loadouts/Weapons/Melee/Sword/PortalSword/BP_PortalSwordPortal.BP_PortalSwordPortal_C" (`self.GetTransform` _returnvalue) "Undefined" "OverrideRootScale" null (`self.PortalTypeToSpawn`) _returnvalue))
  (`/Engine/EditorBlueprintResources/StandardMacros.FlipFlop`
    (:`A`
      (bind _old_portal_s_paired_portal (`self.DeleteOldPortal` (`self.Portal 1`)))
      (set `self.Portal 1` _returnvalue_2)
      (set `/Game/Loadouts/Weapons/Melee/Sword/PortalSword/BP_PortalSwordPortal.Paired Portal` _old_portal_s_paired_portal _returnvalue_2))
    (:`B`
      (bind _old_portal_s_paired_portal_2 (`self.DeleteOldPortal` (`self.Portal 2`)))
      (set `self.Portal 2` _returnvalue_2)
      (set `/Game/Loadouts/Weapons/Melee/Sword/PortalSword/BP_PortalSwordPortal.Paired Portal` _old_portal_s_paired_portal_2 _returnvalue_2)))
  (switch `/Game/Loadouts/Weapons/Melee/Sword/PortalSword/EPortalType` (`self.PortalTypeToSpawn`)
    (:`NewEnumerator0`
      (set `self.PortalTypeToSpawn` "NewEnumerator1"))
    (:`NewEnumerator1`
      (set `self.PortalTypeToSpawn` "NewEnumerator0"))))

(fn `Death Message`
  (params (Killer :type "/Game/UI/In-Game/Chat/STextColor Structure") (Killed :type "/Game/UI/In-Game/Chat/STextColor Structure"))
  (returns (`Death Message` :type "Array of /Game/UI/In-Game/Chat/STextColor Structure"))
  (return (`|MakeArray` Killer (make `/Game/UI/In-Game/Chat/STextColor` "'s ") (make `/Game/UI/In-Game/Chat/STextColor` "Portals" (`self.Color`)) (make `/Game/UI/In-Game/Chat/STextColor` " were too much for ") Killed)))

(fn `DeleteOldPortal`
  (params (`Old Portal` :type "/Game/Loadouts/Weapons/Melee/Sword/PortalSword/BP_PortalSwordPortal Object Reference"))
  (returns (`Old Portal's Paired Portal` :type "/Game/Loadouts/Weapons/Melee/Sword/PortalSword/BP_PortalSwordPortal Object Reference"))
  (locals (`Paired Portal` :type "/Game/Loadouts/Weapons/Melee/Sword/PortalSword/BP_PortalSwordPortal Object Reference"))
  (`/Engine/EditorBlueprintResources/StandardMacros.IsValid` `Old Portal`
    (:`Is Valid`
      (set `local.Paired Portal` (`/Game/Loadouts/Weapons/Melee/Sword/PortalSword/BP_PortalSwordPortal.Paired Portal` `Old Portal`))
      (`self.K2_DestroyActor` `Old Portal`)
      (return (`local.Paired Portal`)))))

(fn `UserConstructionScript`
  (`parent.UserConstructionScript`))