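; BP_BensLightsaber is a melee sword weapon Blueprint for Ben's lightsaber that customizes the kill message.
; Its Death Message function builds colored text segments stating that the killer used the epic power of the weapon on the killed.
; The weapon's name comes from the WeaponName enum and is tinted with its Color variable.
; The event graph holds only disabled default events, and the construction script just calls the parent.
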(fn `Death Message`
  (params (Killer :type "/Game/UI/In-Game/Chat/STextColor Structure") (Killed :type "/Game/UI/In-Game/Chat/STextColor Structure"))
  (returns (`Death Message` :type "Array of /Game/UI/In-Game/Chat/STextColor Structure"))
  (return (`|MakeArray` Killer (make `/Game/UI/In-Game/Chat/STextColor` " used the epic power of ") (make `/Game/UI/In-Game/Chat/STextColor` (`KismetTextLibrary.Conv_StringToText` (`|GetEnumeratorNameAsString` (`self.Weapon Name`))) (`self.Color`)) (make `/Game/UI/In-Game/Chat/STextColor` " on ") Killed)))

(fn `UserConstructionScript`
  (`parent.UserConstructionScript`))