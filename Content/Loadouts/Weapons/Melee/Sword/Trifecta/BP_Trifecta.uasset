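; Trifecta melee weapon that switches between Sword, Spear and Axe forms, each with its own damage, speed, range and movement stats.
; The special input cycles Sword to Spear to Axe, with a short transition lock blocking rapid switching.
; Each switch derives stats from base values cached at BeginPlay, then passes the class and stats through server update events.
; It also supplies a custom kill message.
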(event `self.ReceiveBeginPlay`
  (`parent.ReceiveBeginPlay`)
  (set `self.Base Attack Damage` (`self.Attack Damage`))
  (set `self.Base Attack Speed` (`self.Attack Speed`))
  (set `self.Base Attack Range` (`self.Attack Range`))
  (set `self.Base Movement Speed` (`self.Movement Speed`))
  (`self.Transition to Class` (`self.Starting Class`)))

(event `self.Special Pressed`
  (`self.Transition to Class` (select `/Game/Loadouts/Weapons/EWeaponClass` (`self.Weapon Class`) :`NewEnumerator0` "NewEnumerator3" :`NewEnumerator1` "NewEnumerator0" :`NewEnumerator2` "NewEnumerator0" :`NewEnumerator3` "NewEnumerator1" :`NewEnumerator4` "NewEnumerator0" :`NewEnumerator5` "NewEnumerator0" :`NewEnumerator12` "NewEnumerator0" :`NewEnumerator6` "NewEnumerator0" :`NewEnumerator7` "NewEnumerator0" :`NewEnumerator14` "NewEnumerator0" :`NewEnumerator8` "NewEnumerator0" :`NewEnumerator9` "NewEnumerator0" :`NewEnumerator10` "NewEnumerator0" :`NewEnumerator13` "NewEnumerator0" :!type "/Game/Loadouts/Weapons/EWeaponClass Enum")))

(event `Update Info Server`
  (params (`Atk Damage` :type "Float (double-precision)") (`Atk Speed` :type "Float (double-precision)") (`Atk Range` :type "Float (double-precision)") (`Mvmt Speed` :type "Float (double-precision)"))
  (set `self.Attack Damage` `Atk Damage`)
  (set `self.Attack Speed` `Atk Speed`)
  (set `self.Attack Range` `Atk Range`)
  (set `self.Movement Speed` `Mvmt Speed`))

(event `Transition to Class`
  (params (Class :type "/Game/Loadouts/Weapons/EWeaponClass Enum" :default "NewEnumerator0"))
  (bind _base_attack_damage (`self.Base Attack Damage`))
  (bind _base_attack_speed (`self.Base Attack Speed`))
  (bind _base_attack_range (`self.Base Attack Range`))
  (bind _base_movement_speed (`self.Base Movement Speed`))
  (if (and (not (`self.Is Transitioning`)) (`|EnumInequality` Class (`self.Weapon Class`)))
    (set `self.Is Transitioning` true)
    (bind _output_get (set `self.Weapon Class` Class))
    (`self.Set Class Server` _output_get)
    (`|ExecutionSequence`
      (:`then_0`
        (bind _output_get_2 (set `self.Attack Damage` (select `/Game/Loadouts/Weapons/EWeaponClass` (`self.Weapon Class`) :`NewEnumerator0` _base_attack_damage :`NewEnumerator1` (* _base_attack_damage 1.5) :`NewEnumerator3` (* _base_attack_damage 0.6))))
        (bind _output_get_3 (set `self.Attack Speed` (select `/Game/Loadouts/Weapons/EWeaponClass` (`self.Weapon Class`) :`NewEnumerator0` _base_attack_speed :`NewEnumerator1` (* _base_attack_speed 0.5) :`NewEnumerator3` (* _base_attack_speed 1.2))))
        (bind _output_get_4 (set `self.Attack Range` (select `/Game/Loadouts/Weapons/EWeaponClass` (`self.Weapon Class`) :`NewEnumerator0` _base_attack_range :`NewEnumerator1` (* _base_attack_range 1.4) :`NewEnumerator3` (* _base_attack_range 2.0))))
        (bind _output_get_5 (set `self.Movement Speed` (select `/Game/Loadouts/Weapons/EWeaponClass` (`self.Weapon Class`) :`NewEnumerator0` _base_movement_speed :`NewEnumerator1` (* -1 _base_movement_speed))))
        (`self.Update Info Server` _output_get_2 _output_get_3 _output_get_4 _output_get_5))
      (:`then_1`
        (`KismetSystemLibrary.Delay` 0.8)
        (set `self.Is Transitioning` false)))))

(event `Set Class Server`
  (params (`Weapon Class` :type "/Game/Loadouts/Weapons/EWeaponClass Enum" :default "NewEnumerator0"))
  (set `self.Weapon Class` `Weapon Class`))

(fn `Death Message`
  (params (Killer :type "/Game/UI/In-Game/Chat/STextColor Structure") (Killed :type "/Game/UI/In-Game/Chat/STextColor Structure"))
  (returns (`Death Message` :type "Array of /Game/UI/In-Game/Chat/STextColor Structure"))
  (return (`|MakeArray` Killer (make `/Game/UI/In-Game/Chat/STextColor` "'s ") (make `/Game/UI/In-Game/Chat/STextColor` "Trifecta" (`self.Color`)) (make `/Game/UI/In-Game/Chat/STextColor` " was too versatile for ") Killed)))

(fn `UserConstructionScript`
  (`parent.UserConstructionScript`))