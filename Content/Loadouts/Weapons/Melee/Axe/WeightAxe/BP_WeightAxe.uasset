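; BP_WeightAxe is a melee axe that builds charge levels, starting only while idle with opponents inside its charge collision.
; Owner character animations track charging, which resets on attack, when the last opponent leaves, or on damage with the Branches mod.
; Mod functions adjust stats and set Intimidator, Deposit and Branches flags.
; A Deposited flag doubles the next basic damage calculation, while Intimidator's looping meter-drain timer has an empty loop body.
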(event `self.Pick Up Weapon`
  (params (Player :type "/Game/Loadouts/Characters/BaseClass/BP_CharacterBase Object Reference"))
  (`KismetArrayLibrary.Array_RemoveItem` (`self.Opponents`) Player)
  (`parent.Pick Up Weapon` Player))

(event `self.Charge Collision.OnComponentBeginOverlap`
  (params (OverlappedComponent :type "PrimitiveComponent Object Reference") (OtherActor :type "Actor Object Reference") (OtherComp :type "PrimitiveComponent Object Reference") (OtherBodyIndex :type Integer) (bFromSweep :type Boolean) (SweepResult :type "HitResult Structure (by ref)"))
  (bind _asbp_character_base (cast `/Game/Loadouts/Characters/BaseClass/BP_CharacterBase` OtherActor))
  (if (!= _asbp_character_base (`self.GetOwner`))
    (`KismetArrayLibrary.Array_AddUnique` (`self.Opponents`) _asbp_character_base)))

(event `self.Charge Collision.OnComponentEndOverlap`
  (params (OverlappedComponent :type "PrimitiveComponent Object Reference") (OtherActor :type "Actor Object Reference") (OtherComp :type "PrimitiveComponent Object Reference") (OtherBodyIndex :type Integer))
  (bind _asbp_character_base (cast `/Game/Loadouts/Characters/BaseClass/BP_CharacterBase` OtherActor))
  (bind _returnvalue (`KismetArrayLibrary.Array_RemoveItem` (`self.Opponents`) _asbp_character_base))
  (if _returnvalue
    (if (not (`self.Can Charge`))
      (`self.End Charge`))))

(event `Start Charging`
  (if (`self.Can Charge`)
    (`/Game/Loadouts/Characters/BaseClass/BP_CharacterBase.Weight Axe Charge Anim` (cast `/Game/Loadouts/Characters/BaseClass/BP_CharacterBase` (`self.GetOwner`) :!pure true))
    (if (`self.hasIntimidator`)
      (bind _returnvalue (`KismetSystemLibrary.K2_SetTimerDelegate` (delegate `Drain Blocking Meters`) 0.2 true))
      (set `self.Intimidator Charge Timer` _returnvalue))))

(event `Drain Blocking Meters`
  (for _ (`self.Opponents`)
    _))

(event `Update Charge Level`
  (bind _result (`/Engine/EditorBlueprintResources/StandardMacros.IncrementInt` (`self.Charge Level`))
    (:`  `
      (`KismetSystemLibrary.PrintString` (`KismetStringLibrary.Conv_IntToString` _result))
      (if (>= _result (`self.Max Charge Level`))
        (`/Game/Loadouts/Characters/BaseClass/BP_CharacterBase.Weight Axe Fully Charged` (cast `/Game/Loadouts/Characters/BaseClass/BP_CharacterBase` (`self.GetOwner`) :!pure true))))))

(event `End Charge`
  (bind _asbp_character_base (cast `/Game/Loadouts/Characters/BaseClass/BP_CharacterBase` (`self.GetOwner`)))
  (set `self.Charge Level` 0)
  (`/Game/Loadouts/Characters/BaseClass/BP_CharacterBase.Weight Axe End Charge` _asbp_character_base))

(event `self.On Attack`
  (`parent.On Attack`)
  (`self.End Charge`))

(event `self.On Hit Anything`
  (params (`Hit Result` :type "HitResult Structure"))
  (`parent.On Hit Anything` `Hit Result`)
  (`PlayerCameraManager.StartCameraShake` :`self` (`PlayerController.PlayerCameraManager` (`GameplayStatics.GetPlayerController` 0)) :`ShakeClass` "/Game/VisualEffects/CameraShake/GenericCameraShake.GenericCameraShake_C"))

(event `self.On Owning Player Damaged`
  (params (Damage :type "/Game/HealthInterface/Dmg Structure"))
  (`parent.On Owning Player Damaged` Damage)
  (if (`self.hasBranches`)
    (`self.End Charge`)))

(fn `Calculate Basic Flat Attack Damage`
  (returns (`Final Flat Damage` :type "Float (double-precision)"))
  (bind _final_flat_damage (`parent.Calculate Basic Flat Attack Damage`))
  (if (`self.deposited`)
    (set `self.deposited` false)
    (return (* 2 _final_flat_damage))
    (else
      (return _final_flat_damage))))

(fn `Can Charge`
  (returns (Return :type Boolean))
  (bind _asbp_character_base (cast `/Game/Loadouts/Characters/BaseClass/BP_CharacterBase` (`self.GetOwner`))
    (:`then`
      (return (and (> (`KismetArrayLibrary.Array_Length` (`self.Opponents`)) 0) (select `/Game/Loadouts/Weapons/Melee/Axe/WeightAxe/EWeightAxeState` (`/Game/Loadouts/Characters/BaseClass/BP_CharacterBase.WeightAxeCharge` _asbp_character_base) :`NewEnumerator0` true))))
    (:`CastFailed`
      (return false))))

(fn `Death Message`
  (params (Killer :type "/Game/UI/In-Game/Chat/STextColor Structure") (Killed :type "/Game/UI/In-Game/Chat/STextColor Structure"))
  (returns (`Death Message` :type "Array of /Game/UI/In-Game/Chat/STextColor Structure"))
  (return (`|MakeArray` Killer (make `/Game/UI/In-Game/Chat/STextColor` " Weighed" (`self.Color`)) (make `/Game/UI/In-Game/Chat/STextColor` " down ") Killed)))

(fn `Mod_10`
  (set `self.Attack Damage` (- (`self.Attack Damage`) 8.0))
  (set `self.Charge Speed` (* 2 (`self.Charge Speed`))))

(fn `Mod_11`
  (set `self.Charge Speed` (* 2 (`self.Charge Speed`)))
  (set `self.Movement Speed` (+ (`self.Movement Speed`) 0.02))
  (set `self.hasBranches` true))

(fn `Mod_12`
  (set `self.hasDeposit` true))

(fn `Mod_9`
  (set `self.hasIntimidator` true)
  (`self.Fix Mod Mesh Visibility` (`self.Intimidator`)))

(fn `UserConstructionScript`
  (`self.Add Meshes` (`|MakeArray` (`self.Speed Charger`) (`self.Intimidator`) (`self.Deposit`) (`self.Branches`) :!type "PrimitiveComponent Object Reference"))
  (`parent.UserConstructionScript`))