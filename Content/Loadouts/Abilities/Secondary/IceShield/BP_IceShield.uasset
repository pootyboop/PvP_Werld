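; BP_IceShield is a secondary-ability ice shield actor that absorbs damage for a limited time.
; On BeginPlay, a timeline scales the shield up from zero, while ability level increases its health and lifetime.
; Damage events subtract health; the shield destroys itself when health equals exactly zero or the delay expires.
; GetHealthAsRatio is a stub returning zero, and an ability-level branch is left unconnected.
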(event `self.ReceiveBeginPlay`
  (set `self.Health` (+ (`self.Health`) (`KismetMathLibrary.Conv_IntToDouble` (* (`self.Ability Level`) 10))))
  (`|ExecutionSequence`
    (:`then_0`
      (bind (_direction _lerp) (`Timeline|IceShieldAnim` :!via `PlayFromStart`)
        (:`Update`
          (`SceneComponent.SetWorldScale3D` (`self.Ice Shield`) (`KismetMathLibrary.VLerp` (0.0 0.0 0.0) (1.0 1.0 1.0) _lerp)))))
    (:`then_1`
      (`KismetSystemLibrary.Delay` (+ 5.0 (`KismetMathLibrary.Conv_IntToDouble` (* (`self.Ability Level`) 3))))
      (`self.Destroy`))))

(event `Destroy`
  (`self.K2_DestroyActor`))

(event `/Game/HealthInterface/BPI_HealthInterface.Damage`
  (params (`Damage Information` :type "/Game/HealthInterface/Dmg Structure"))
  (bind _output_get (set `self.Health` (- (`self.Health`) `Damage Information_Damage_2_390607314C7D738086617A977C8A56C6`)))
  (if (== _output_get 0.0)
    (`self.Destroy`)))

(fn `GetHealthAsRatio`
  (returns (`Health As Ratio` :type "Float (double-precision)"))
  (return 0.0))

(fn `UserConstructionScript`)