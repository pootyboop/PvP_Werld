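; BP_MainPC is the player controller, handling loadout hand-off, the end-of-game screen and the death camera fade.
; On BeginPlay, the locally controlled player reads its equipped loadout from the save game and passes it to SetLoadoutServer.
; EndGameMulti shows local players W_EndScreen with the winner's name and color.
; It also has weapon-destruction and player-state helpers, while chat box, weapon-cleanup and simulated-lag chains are left disconnected.
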(event `self.ReceiveBeginPlay`
  (`self.Get Save Game Multi`))

(event `Get Save Game Multi`
  (bind _returnvalue (`self.K2_GetPawn`))
  (`/Engine/EditorBlueprintResources/StandardMacros.IsValid` _returnvalue
    (:`Is Valid`
      (if (`Pawn.IsLocallyControlled` _returnvalue)
        (`self.Set Loadout Server` (`/Game/Saving/BP_SaveGame.Get Currently Equipped Loadout` (`/Game/BPFunctionLibrary.Get Save Game`)))))))

(event `Set Loadout Server`
  (params (Loadout :type "/Game/Loadouts/sLoadout Structure"))
  (set `self.Loadout` Loadout))

(event `self.ReceiveEndPlay`
  (params (EndPlayReason :type "EEndPlayReason Enum" :default "Destroyed")))

(event `Destroy Weapons Server`
  (params (Player :type "/Game/Loadouts/Characters/BaseClass/BP_CharacterBase Object Reference"))
  (`self.Destroy Weapons` Player))

(event `End Game Multi`
  (params (`Winner Player State` :type "/Game/Loadouts/Characters/BaseClass/BP_MainPlayerState Object Reference"))
  (bind _asbp_character_base (cast `/Game/Loadouts/Characters/BaseClass/BP_CharacterBase` (`PlayerState.PawnPrivate` `Winner Player State`) :!pure true))
  (if (`Pawn.IsLocallyControlled` (`self.K2_GetPawn`))
    (bind _returnvalue (`|CreateWidget` "/Game/UI/In-Game/Gamemode/W_EndScreen.W_EndScreen_C" self (`KismetTextLibrary.Conv_StringToText` (`/Game/Loadouts/Characters/BaseClass/BP_CharacterBase.Player Name` _asbp_character_base)) (`/Game/Loadouts/Characters/BaseClass/BP_CharacterBase.Color` _asbp_character_base)))
    (`UserWidget.AddToViewport` _returnvalue 0)))

(event `Death Camera Fade`
  (params (Stop :type Boolean))
  (bind _returnvalue (`GameplayStatics.GetPlayerCameraManager` 0))
  (if Stop
    (`PlayerCameraManager.StopCameraFade` _returnvalue)
    (else
      (`PlayerCameraManager.StartCameraFade` :`self` _returnvalue :`ToAlpha` 1.0 :`Duration` 0.5 :`bHoldWhenFinished` true))))

(fn `Destroy Weapons`
  (params (Player :type "/Game/Loadouts/Characters/BaseClass/BP_CharacterBase Object Reference"))
  (`self.K2_DestroyActor` (`/Game/Loadouts/Characters/BaseClass/BP_CharacterBase.First Weapon` Player))
  (`self.K2_DestroyActor` (`/Game/Loadouts/Characters/BaseClass/BP_CharacterBase.Second Weapon` Player)))

(fn `Get Player State`
  (returns (`Main Player State` :type "/Game/Loadouts/Characters/BaseClass/BP_MainPlayerState Object Reference") (bSuccess :type Boolean))
  (bind (_asbp_main_player_state _bsuccess) (cast `/Game/Loadouts/Characters/BaseClass/BP_MainPlayerState` (`self.PlayerState`) :!pure true))
  (return _asbp_main_player_state _bsuccess))

(fn `UserConstructionScript`)