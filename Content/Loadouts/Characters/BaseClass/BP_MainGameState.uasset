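; Main game state providing shared helpers for area-of-effect hit detection and player spawning.
; SpawnAOE sphere-overlaps pawns implementing the health interface and reports hits through a caller-supplied delegate, bound only for that call.
; Optional line-of-sight traces to the bounds center and eight offset points count a hit on the first unblocked trace, with optional debug drawing.
; SpawnPlayer spawns the controller's loadout character, possesses it, teleports it into place and sets the controller's gamemode name.
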(fn `GetBoxCorners`
  (params (Origin :type "Vector Structure") (BoxExtent :type "Vector Structure"))
  (returns (Corners :type "Array of Vector Structure"))
  (bind (_boxextent_x _boxextent_y _boxextent_z) (`KismetMathLibrary.BreakVector` (`local.BoxExtent`)))
  (bind (_boxextent_x_2 _boxextent_y_2 _boxextent_z_2) (`KismetMathLibrary.BreakVector` (`local.BoxExtent`)))
  (bind (_boxextent_x_3 _boxextent_y_3 _boxextent_z_3) (`KismetMathLibrary.BreakVector` (`local.BoxExtent`)))
  (bind (_boxextent_x_4 _boxextent_y_4 _boxextent_z_4) (`KismetMathLibrary.BreakVector` (`local.BoxExtent`)))
  (bind (_boxextent_x_5 _boxextent_y_5 _boxextent_z_5) (`KismetMathLibrary.BreakVector` (`local.BoxExtent`)))
  (bind (_boxextent_x_6 _boxextent_y_6 _boxextent_z_6) (`KismetMathLibrary.BreakVector` (`local.BoxExtent`)))
  (bind (_boxextent_x_7 _boxextent_y_7 _boxextent_z_7) (`KismetMathLibrary.BreakVector` (`local.BoxExtent`)))
  (bind (_boxextent_x_8 _boxextent_y_8 _boxextent_z_8) (`KismetMathLibrary.BreakVector` (`local.BoxExtent`)))
  (return (`|MakeArray` (`local.Origin`) (+ (`local.Origin`) (`KismetMathLibrary.MakeVector` _boxextent_x 0.0 _boxextent_z)) (+ (`local.Origin`) (`KismetMathLibrary.MakeVector` (* -1 _boxextent_x_2) 0.0 _boxextent_z_2)) (+ (`local.Origin`) (`KismetMathLibrary.MakeVector` 0.0 _boxextent_y_4 _boxextent_z_4)) (+ (`local.Origin`) (`KismetMathLibrary.MakeVector` 0.0 (* -1 _boxextent_x_3) _boxextent_z_3)) (+ (`local.Origin`) (`KismetMathLibrary.MakeVector` _boxextent_x_8 0.0 (* -1 _boxextent_z_8))) (+ (`local.Origin`) (`KismetMathLibrary.MakeVector` (* -1 _boxextent_x_7) 0.0 (* -1 _boxextent_z_7))) (+ (`local.Origin`) (`KismetMathLibrary.MakeVector` 0.0 _boxextent_y_6 (* -1 _boxextent_z_6))) (+ (`local.Origin`) (`KismetMathLibrary.MakeVector` 0.0 (* -1 _boxextent_x_5) (* -1 _boxextent_z_5))))))

(fn `Spawn AOE`
  (params (Location :type "Vector Structure") (Radius :type "Float (double-precision)" :default 400.0) (RequireLOS :type Boolean :default true) (`AOE Instigator` :type "Actor Object Reference") (`Hit Delegate` :type "Delegate (by ref)") (DrawDebugDuration :type "Float (double-precision)" :default 0.0) (`Debug Color` :type "LinearColor Structure"))
  (locals (`Current Actor` :type "Actor Object Reference"))
  (bind (_origin _boxextent) (`self.GetActorBounds` (`local.Current Actor`) true true))
  (add `self.AOE Hit Delegate` `Hit Delegate`)
  (`|ExecutionSequence`
    (:`then_0`
      (if (> (`local.DrawDebugDuration`) 0.0)
        (`KismetSystemLibrary.DrawDebugSphere` (`local.Location`) (`local.Radius`) 16 (`local.Debug Color`) (`local.DrawDebugDuration`) 2.0))
      (bind _outactors (`KismetSystemLibrary.SphereOverlapActors` (`local.Location`) (`local.Radius`) (`|MakeArray` "ObjectTypeQuery3" :!type "EObjectTypeQuery Enum") "/Script/Engine.Actor" (`|MakeArray` (`local.AOE Instigator`))))
      (for _array_element _outactors
        (bind _output_get (set `local.Current Actor` _array_element))
        (if (`KismetSystemLibrary.DoesImplementInterface` _output_get "/Game/HealthInterface/BPI_HealthInterface.BPI_HealthInterface_C")
          (if (`local.RequireLOS`)
            (bind _corners (`self.GetBoxCorners` _origin _boxextent))
            (for _array_element_2 _corners
              (bind (_outhit _returnvalue) (`KismetSystemLibrary.LineTraceSingle` (`local.Location`) _array_element_2 "TraceTypeQuery1" false (`|MakeArray` (`local.AOE Instigator`)) (select `bool` (> (`local.DrawDebugDuration`) 0.0) :`true` "ForDuration" :!type "EDrawDebugTrace Enum") true (struct :`R` 1.0 :`A` 1.0) (struct :`G` 1.0 :`A` 1.0) (`local.DrawDebugDuration`)))
              (if (not _returnvalue)
                (`self.AOE Hit Delegate` (`local.Current Actor`))
                (break)))
            (else
              (`self.AOE Hit Delegate` (`local.Current Actor`)))))))
    (:`then_1`
      (remove `self.AOE Hit Delegate` (`local.Hit Delegate`)))))

(fn `Spawn Player`
  (params (SpawnTransform :type "Transform Structure") (`Main PC` :type "/Game/Loadouts/Characters/BaseClass/BP_MainPC Object Reference") (`Gamemode Name` :type "/Game/Gamemodes/EGamemodeName Enum" :default "NewEnumerator0"))
  (locals (Character :type "/Game/Loadouts/Characters/BaseClass/BP_CharacterBase Object Reference"))
  (bind (_loadout_loadoutname _loadout_loadoutcolor _loadout_character) (break `/Game/Loadouts/sLoadout` (`/Game/Loadouts/Characters/BaseClass/BP_MainPC.Loadout` `Main PC`)))
  (bind _returnvalue (`|SpawnActorFromClass` _loadout_character SpawnTransform "Undefined" "OverrideRootScale" null false false null))
  (bind _output_get (set `local.Character` _returnvalue))
  (`Controller.Possess` (`local.Main PC`) _output_get)
  (`self.K2_SetActorTransform` (`local.Character`) (`local.SpawnTransform`) false true)
  (set `/Game/Loadouts/Characters/BaseClass/BP_MainPC.Gamemode Name` (`local.Gamemode Name`) (`local.Main PC`)))

(fn `UserConstructionScript`)