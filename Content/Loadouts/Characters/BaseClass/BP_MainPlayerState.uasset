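; Player state Blueprint holding a player's name, color, score, kills and deaths, with name and color loaded from the save game.
; Chat messages pass through server and multicast events to the locally controlled character's chat box.
; Score and K/D updates write to character scoreboard entries matched by player name.
; Setting the score also calls the game mode's Win once it reaches ScoreToWin.
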(event `self.ReceiveBeginPlay`
  (bind _save_game (`/Game/BPFunctionLibrary.Get Save Game`))
  (set `self.Player Name` (`/Game/Saving/BP_SaveGame.Player Name` _save_game))
  (set `self.Color` (`/Game/Saving/BP_SaveGame.Color` _save_game)))

(event `Send Chat Message`
  (params (Message :type "Array of /Game/UI/In-Game/Chat/STextColor Structure") (isDeathMessage :type Boolean))
  (`self.Send Chat Message Server` Message isDeathMessage))

(event `Send Chat Message Server`
  (params (Message :type "Array of /Game/UI/In-Game/Chat/STextColor Structure") (isDeathMessage :type Boolean))
  (`self.Send Chat Message Multi` Message isDeathMessage))

(event `Send Chat Message Multi`
  (params (Message :type "Array of /Game/UI/In-Game/Chat/STextColor Structure") (isDeathMessage :type Boolean))
  (bind _asbp_character_base (cast `/Game/Loadouts/Characters/BaseClass/BP_CharacterBase` (`Controller.K2_GetPawn` (`GameplayStatics.GetPlayerController` 0))))
  (if (`Pawn.IsLocallyControlled` _asbp_character_base)
    (`/Game/Loadouts/Characters/BaseClass/BP_CharacterBase.Add Message to Chat Box` _asbp_character_base Message isDeathMessage)))

(fn `Get Scoreboard Slots`
  (returns (`Scoreboard Slot` :type "Array of /Game/UI/In-Game/Scoreboard/W_ScoreboardPlayerSlot Object Reference"))
  (locals (`Valid Slots` :type "Array of /Game/UI/In-Game/Scoreboard/W_ScoreboardPlayerSlot Object Reference"))
  (bind _outactors (`GameplayStatics.GetAllActorsOfClass` "/Game/Loadouts/Characters/BaseClass/BP_CharacterBase.BP_CharacterBase_C"))
  (for _array_element _outactors
    (bind _scoreboard (`/Game/Loadouts/Characters/BaseClass/BP_CharacterBase.Scoreboard` _array_element)
      (:`then`
        (for _array_element_2 (`/Game/UI/In-Game/Scoreboard/W_Scoreboard.Scoreboard Players` _scoreboard)
          (if (`KismetStringLibrary.EqualEqual_StrStr` (`KismetTextLibrary.Conv_TextToString` (`/Game/UI/In-Game/Scoreboard/W_ScoreboardPlayerSlot.Player Name` _array_element_2)) (`self.Player Name`))
            (`KismetArrayLibrary.Array_AddUnique` (`local.Valid Slots`) _array_element_2)))
        (return (`local.Valid Slots`)))
      (:`else`))))

(fn `Increment Deaths`
  (`/Engine/EditorBlueprintResources/StandardMacros.IncrementInt` (`self.Deaths`)
    (:`  `
      (`self.Update Scoreboard K/D`))))

(fn `Increment Kills`
  (`/Engine/EditorBlueprintResources/StandardMacros.IncrementInt` (`self.Kills`)
    (:`  `
      (`self.Update Scoreboard K/D`))))

(fn `Set Game Score`
  (params (`New Score` :type "Float (double-precision)") (PC :type "/Game/Loadouts/Characters/BaseClass/BP_MainPC Object Reference"))
  (set `self.Game Score` `New Score`)
  (`|ExecutionSequence`
    (:`then_0`
      (bind _outactors (`GameplayStatics.GetAllActorsOfClass` "/Game/Loadouts/Characters/BaseClass/BP_CharacterBase.BP_CharacterBase_C"))
      (for _array_element _outactors
        (bind _scoreboard (`/Game/Loadouts/Characters/BaseClass/BP_CharacterBase.Scoreboard` _array_element)
          (:`then`
            (for _array_element_2 (`/Game/UI/In-Game/Scoreboard/W_Scoreboard.Scoreboard Players` _scoreboard)
              (if (`KismetStringLibrary.EqualEqual_StrStr` (`KismetTextLibrary.Conv_TextToString` (`/Game/UI/In-Game/Scoreboard/W_ScoreboardPlayerSlot.Player Name` _array_element_2)) (`self.Player Name`))
                (bind _output_get (set `/Game/UI/In-Game/Scoreboard/W_ScoreboardPlayerSlot.Score` (`self.Game Score`) _array_element_2))
                (`KismetSystemLibrary.PrintString` (`KismetStringLibrary.Conv_DoubleToString` _output_get))
                (else
                  (`KismetSystemLibrary.PrintString` "FAILED")))))
          (:`else`))))
    (:`then_1`
      (bind _asbp_main_game_mode (cast `/Game/Gamemodes/BP_MainGameMode` (`GameplayStatics.GetGameMode`)))
      (if (>= (`self.Game Score`) (`/Game/Gamemodes/BP_MainGameMode.Score to Win` _asbp_main_game_mode))
        (`/Game/Gamemodes/BP_MainGameMode.Win` _asbp_main_game_mode self)))))

(fn `Update Scoreboard K/D`
  (for _array_element (`self.Get Scoreboard Slots`)
    (set `/Game/UI/In-Game/Scoreboard/W_ScoreboardPlayerSlot.Kill/Death Ratio` (`/Game/BPFunctionLibrary.Calculate Kill/ Death Ratio` (`self.Kills`) (`self.Deaths`)) _array_element)))

(fn `UserConstructionScript`)