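; Rocketeer playable character that adds a fuel-limited jetpack, with a HUD widget showing boost.
; Tick drains boost to apply repeated LaunchCharacter thrust while jump is held airborne, outside a brief post-jump delay, so rates are per-frame.
; Grounding, mantling and wall jumps refill boost, scaled by the Focus perk.
; Effects and thrust run immediately on the owning client, then replay on others through server-to-multicast events that skip the local player.
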(event `Create Rocketeer Widget`
  (bind _returnvalue (`|CreateWidget` "/Game/UI/In-Game/Character/W_RocketeerInfo.W_RocketeerInfo_C" (`GameplayStatics.GetPlayerController` 0)))
  (`/Engine/EditorBlueprintResources/StandardMacros.IsValid` _returnvalue
    (:`Is Valid`
      (bind _output_get (set `self.Rocketeer Widget` _returnvalue))
      (`UserWidget.AddToViewport` _output_get 0))))

(event `Activate Jetpack Server`
  (`self.Activate Jetpack Multi`))

(event `Activate Jetpack Multi`
  (if (not (`self.IsLocallyControlled`))
    (`ActorComponent.Activate` (`self.Jetpack`) false :!label _label)
    (`ActorComponent.Activate` (`self.Jetpack1`) false)))

(event `self.ReceiveTick`
  (params (DeltaSeconds :type "Float (single-precision)"))
  (bind (_returnvalue_x _returnvalue_y _returnvalue_z) (`KismetMathLibrary.BreakVector` (`self.GetVelocity`)))
  (bind _is_using_jetpack (`self.Is Using Jetpack`))
  (`parent.ReceiveTick` DeltaSeconds)
  (if (or (`NavMovementComponent.IsMovingOnGround` (`self.GetMovementComponent`)) (select `/Game/Loadouts/Characters/BaseClass/EMovementState` (`self.MovementState`) :`NewEnumerator4` true))
    (`self.Add to Jetpack Boost` 1)
    (elif (and (`self.isHoldingJump`) (> (`self.Jetpack Boost`) 0) (select `/Game/Loadouts/Characters/BaseClass/EMovementState` (`self.MovementState`) :`NewEnumerator0` true :`NewEnumerator3` true) (not (`self.Is Jumping`)))
      (if _is_using_jetpack
        (`|ExecutionSequence` :!label _label_2
          (:`then_0`
            (`self.LaunchCharacter` (`KismetMathLibrary.MakeVector` 0.0 0.0 (+ (/ _returnvalue_z -10.0) 80.0)) :!label _label_3))
          (:`then_1`
            (`self.Rocketeer Boost Server`)
            (`/Engine/EditorBlueprintResources/StandardMacros.DecrementInt` (`self.Jetpack Boost`)
              (:`  `
                (bind _rocketeer_widget (`self.Rocketeer Widget`)
                  (:`then`
                    (`/Game/UI/In-Game/Character/W_RocketeerInfo.Update Info` _rocketeer_widget (`self.Jetpack Boost`) (`self.Max Jetpack Boost`))
                    (bind _rocketeer_widget_2 (`self.Rocketeer Widget`)
                      (:`then`
                        (if (and (`|EnumInequality` (`Widget.GetVisibility` _rocketeer_widget_2) "Visible") (< (`self.Jetpack Boost`) (`KismetMathLibrary.FTrunc` (* (`self.Max Jetpack Boost`) 0.8))))
                          (bind _rocketeer_widget_3 (`self.Rocketeer Widget`)
                            (:`then`
                              (`/Game/UI/In-Game/Character/W_RocketeerInfo.Update Info` _rocketeer_widget_3 (`self.Jetpack Boost`) 0)
                              (switch `/Game/Loadouts/Characters/BaseClass/EMovementState` (`self.MovementState`)
                                (:`NewEnumerator2`
                                  (`self.EndSlide`))))
                            (:`else`))))
                      (:`else`)))
                  (:`else`))))))
        (else
          (set `self.Is Using Jetpack` true)
          (`|ExecutionSequence`
            (:`then_0`
              (goto _label))
            (:`then_1`
              (`self.Activate Jetpack Server`))
            (:`then_2`
              (goto _label_2)))))
      (elif _is_using_jetpack
        (set `self.Is Using Jetpack` false)
        (`|ExecutionSequence`
          (:`then_0`
            (`ActorComponent.Deactivate` (`self.Jetpack`) :!label _label_4)
            (`ActorComponent.Deactivate` (`self.Jetpack1`)))
          (:`then_1`
            (`self.Deactivate Jetpack Server`)))))))

(event `Rocketeer Boost Server`
  (`self.Rocketeer Boost Multi`))

(event `Rocketeer Boost Multi`
  (if (not (`self.IsLocallyControlled`))
    (goto _label_3)))

(event `Deactivate Jetpack Server`
  (`self.Deactivate Jetpack Multi`))

(event `Deactivate Jetpack Multi`
  (if (not (`self.IsLocallyControlled`))
    (goto _label_4)))

(event `self.OnJumped`
  (set `self.Is Jumping` true :!label _label_5)
  (`KismetSystemLibrary.RetriggerableDelay` 0.3)
  (set `self.Is Jumping` false))

(event `self.On Wall Jump`
  (`self.Add to Jetpack Boost` 30)
  (goto _label_5))

(event `self.Kill Owning Client`
  (params (`Last Damage` :type "/Game/HealthInterface/Dmg Structure"))
  (bind _rocketeer_widget (`self.Rocketeer Widget`)
    (:`then`
      (`Widget.RemoveFromParent` _rocketeer_widget)
      (`parent.Kill Owning Client` `Last Damage`))
    (:`else`)))

(fn `Add to Jetpack Boost`
  (params (Amount :type Integer))
  (if (< (`self.Jetpack Boost`) (`self.Max Jetpack Boost`))
    (set `self.Jetpack Boost` (`KismetMathLibrary.Clamp` (+ (* Amount (+ (`self.Get Number of Perk` "Focus") 1)) (`self.Jetpack Boost`)) 0 (`self.Max Jetpack Boost`)))
    (bind _rocketeer_widget (`self.Rocketeer Widget`)
      (:`then`
        (`/Game/UI/In-Game/Character/W_RocketeerInfo.Update Info` _rocketeer_widget (`self.Jetpack Boost`) (`self.Max Jetpack Boost`)))
      (:`else`))))

(fn `UserConstructionScript`
  (`parent.UserConstructionScript`))