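; BP_Shroom is the Shroom character Blueprint, whose only custom logic overrides how status effects are added.
; AddStatusEffect copies the incoming effect into StatusDamage and removes entries of one enum type from its effect list while looping over it.
; It then calls the parent with the original StatusEffect input rather than the filtered StatusDamage.
; The event graph holds only disabled default nodes, and construction just calls the parent.
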(fn `Add Status Effect`
  (params (`Status Effect` :type "/Game/HealthInterface/Dmg Structure (by ref)"))
  (locals (`Status Damage` :type "/Game/HealthInterface/Dmg Structure"))
  (bind _output_get (set `local.Status Damage` `Status Effect`))
  (bind (_damage _damagetype _instigator _literaldamagedealer _statuseffects) (break `/Game/HealthInterface/Dmg` _output_get))
  (for _array_element _statuseffects
    (if (`|EnumEquality` (`.Name_8_83DCBC7D429B1491E3137F9AC8E7A4D4` (break `/Game/StatusEffects/StatusEffect` _array_element)) "NewEnumerator0")
      (`KismetArrayLibrary.Array_RemoveItem` _statuseffects _array_element)))
  (`parent.Add Status Effect` (`local.Status Effect`))
  (return))

(fn `UserConstructionScript`
  (`parent.UserConstructionScript`))