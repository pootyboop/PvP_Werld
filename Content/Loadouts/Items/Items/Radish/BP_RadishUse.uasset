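; Use logic for the Radish loadout item, which heals its user and nearby teammates.
; UseItem only acts when the player is below max health, applying HealAmount and decrementing the item count.
; Unless the player is on one particular team, it then has BP_MainGameState spawn an AOE, without line of sight, at its own location.
; The AOE's hit delegate heals same-team characters for half of HealAmount.
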(event `self.Use Item`
  (params (Player :type "/Game/Loadouts/Characters/BaseClass/BP_CharacterBase Object Reference") (`Item #` :type Integer))
  (if (!= (`/Game/Loadouts/Characters/BaseClass/BP_CharacterBase.Health` Player) (`/Game/Loadouts/Characters/BaseClass/BP_CharacterBase.Max Health` Player))
    (`/Game/HealthInterface/BPI_HealthInterface.Heal` Player (`self.Heal Amount`))
    (`self.Decrement Item Count` Player `Item #`)
    (if (`|EnumInequality` (`/Game/Loadouts/Characters/BaseClass/BP_CharacterBase.Team` Player) "NewEnumerator2")
      (bind _asbp_main_game_state (cast `/Game/Loadouts/Characters/BaseClass/BP_MainGameState` (`GameplayStatics.GetGameState`)))
      (`/Game/Loadouts/Characters/BaseClass/BP_MainGameState.Spawn AOE` _asbp_main_game_state (`self.K2_GetActorLocation`) 400.0 false self (delegate `Heal Nearby Teammates`) 2.0 (struct :`R` 0.034433 :`G` 0.484375 :`A` 1.0)))))

(event `Heal Nearby Teammates`
  (params (`Hit Actor` :type "Actor Object Reference"))
  (bind _asbp_character_base (cast `/Game/Loadouts/Characters/BaseClass/BP_CharacterBase` `Hit Actor` :!pure true))
  (if (`|EnumEquality` (`/Game/Loadouts/Characters/BaseClass/BP_CharacterBase.Team` _asbp_character_base) (`/Game/Loadouts/Characters/BaseClass/BP_CharacterBase.Team` (stale `self.Use Item` Player)))
    (`/Game/HealthInterface/BPI_HealthInterface.Heal` _asbp_character_base (/ (`self.Heal Amount`) 2.0))))

(fn `UserConstructionScript`
  (`parent.UserConstructionScript`))