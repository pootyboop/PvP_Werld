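; BP_GrenadeBase is a base Blueprint for thrown or launched grenade projectiles.
; On BeginPlay it applies its Velocity variable to ProjectileMovement and makes the SkeletalMesh ignore the instigator while moving.
; The Hit event flags the first impact, then sets HitTwice and calls HitTwiceEvent on every later one.
; HitTwiceEvent is empty here, which leaves a hook for child grenades.
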(event `self.ReceiveBeginPlay`
  (set `MovementComponent.Velocity` (`self.Velocity`) (`self.ProjectileMovement`))
  (`PrimitiveComponent.IgnoreActorWhenMoving` (`self.SkeletalMesh`) (`self.GetInstigator`) true))

(event `self.ReceiveHit`
  (params (MyComp :type "PrimitiveComponent Object Reference") (Other :type "Actor Object Reference") (OtherComp :type "PrimitiveComponent Object Reference") (bSelfMoved :type Boolean) (HitLocation :type "Vector Structure") (HitNormal :type "Vector Structure") (NormalImpulse :type "Vector Structure") (Hit :type "HitResult Structure (by ref)"))
  (if (`self.hit`)
    (set `self.hitTwice` true)
    (`self.Hit Twice Event`)
    (else
      (set `self.hit` true))))

(event `Hit Twice Event`)

(fn `UserConstructionScript`)