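; BP_GravityGrenadeUse is the use-action Blueprint for the Gravity Grenade loadout item, throwing a grenade when the player uses the item.
; UseItem calls the player's GrenadeServer with a spawn transform just in front of the camera, a fixed-speed velocity along the view direction and the player as instigator.
; It then decrements the item count, leaving the grenade spawn and behavior to code outside this Blueprint.
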(event `self.Use Item`
  (params (Player :type "/Game/Loadouts/Characters/BaseClass/BP_CharacterBase Object Reference") (`Item #` :type Integer))
  (bind _camera (`/Game/Loadouts/Characters/BaseClass/BP_CharacterBase.Camera` Player))
  (bind _returnvalue (`SceneComponent.GetForwardVector` _camera))
  (`/Game/Loadouts/Characters/BaseClass/BP_CharacterBase.Grenade Server` Player (`KismetMathLibrary.MakeTransform` (+ (`SceneComponent.K2_GetComponentLocation` _camera) _returnvalue) (`SceneComponent.K2_GetComponentRotation` _camera)) (* _returnvalue 2200.0) Player)
  (`self.Decrement Item Count` Player `Item #`))

(fn `UserConstructionScript`
  (`parent.UserConstructionScript`))