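; BP_LoadoutComponent is an interactable actor that shows an interaction prompt when a nearby local player looks at it.
; Sphere overlaps maintain a NearbyPlayers list of BP_CharacterBase, which gates both look events.
; LookedAt creates a screen-space widget component at runtime, using getter functions for text and attach point.
; LookedAwayFrom destroys it only while the player is still listed, and leaving the sphere does not remove it.
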(event `Looked At`
  (params (Player :type "/Game/Loadouts/Characters/BaseClass/BP_CharacterBase Object Reference"))
  (bind _returnvalue (`Pawn.GetController` Player))
  (`self.Is Player Nearby` Player
    (:`true`
      (`/Engine/EditorBlueprintResources/StandardMacros.IsValid` _returnvalue
        (:`Is Valid`
          (if (`Controller.IsLocalPlayerController` _returnvalue)
            (`self.Interaction Widget Component`
              (:`then`)
              (:`else`
                (bind _returnvalue_2 (`|CreateWidget` "/Game/InteractionInterface/InteractionWidget.InteractionWidget_C" (cast `PlayerController` _returnvalue :!pure true) (`self.GetInteractionText`)))
                (bind _returnvalue_3 (`AddComponent|NODE_AddWidgetComponent-0`))
                (bind _output_get (set `self.Interaction Widget Component` _returnvalue_3))
                (`WidgetComponent.SetWidget` _output_get _returnvalue_2)
                (`WidgetComponent.SetWidgetSpace` _output_get "Screen")
                (`WidgetComponent.SetDrawAtDesiredSize` _output_get false)
                (`PrimitiveComponent.SetCollisionEnabled` _output_get "NoCollision")
                (`SceneComponent.K2_AttachToComponent` _output_get (`self.GetInteractionTextAttach`) "None" "SnapToTarget" "SnapToTarget" "SnapToTarget" true)))))))))

(event `Looked Away From`
  (params (Player :type "/Game/Loadouts/Characters/BaseClass/BP_CharacterBase Object Reference"))
  (`self.Is Player Nearby` Player
    (:`true`
      (`self.Destroy Interaction Widget`))))

(event `self.Sphere.OnComponentBeginOverlap`
  (params (OverlappedComponent :type "PrimitiveComponent Object Reference") (OtherActor :type "Actor Object Reference") (OtherComp :type "PrimitiveComponent Object Reference") (OtherBodyIndex :type Integer) (bFromSweep :type Boolean) (SweepResult :type "HitResult Structure (by ref)"))
  (bind _asbp_character_base (cast `/Game/Loadouts/Characters/BaseClass/BP_CharacterBase` OtherActor))
  (`KismetArrayLibrary.Array_AddUnique` (`self.Nearby Players`) _asbp_character_base))

(event `self.Sphere.OnComponentEndOverlap`
  (params (OverlappedComponent :type "PrimitiveComponent Object Reference") (OtherActor :type "Actor Object Reference") (OtherComp :type "PrimitiveComponent Object Reference") (OtherBodyIndex :type Integer))
  (bind _asbp_character_base (cast `/Game/Loadouts/Characters/BaseClass/BP_CharacterBase` OtherActor))
  (`KismetArrayLibrary.Array_RemoveItem` (`self.Nearby Players`) _asbp_character_base))

(fn `Check If Player Nearby`
  (params (Player :type "/Game/Loadouts/Characters/BaseClass/BP_CharacterBase Object Reference"))
  (returns (Return :type Boolean))
  (`self.Is Player Nearby` Player
    (:`true`
      (return true))
    (:`false`
      (return false))))

(fn `Destroy Interaction Widget`
  (bind _interaction_widget_component (`self.Interaction Widget Component`)
    (:`then`
      (`ActorComponent.K2_DestroyComponent` _interaction_widget_component))
    (:`else`)))

(fn `GetInteractionText`
  (returns (Text :type Text))
  (return "Interact"))

(fn `GetInteractionTextAttach`
  (returns (AttachComponent :type "SceneComponent Object Reference"))
  (return (`self.DefaultSceneRoot`)))

(fn `UserConstructionScript`)