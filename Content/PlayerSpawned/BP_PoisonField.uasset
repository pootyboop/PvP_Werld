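; Player-spawned poison field actor that deals damage over time in a growing area.
; Each Tick it asks BP_MainGameState to spawn an AOE at its location, without a line-of-sight check and with a green debug draw.
; The DamageAOE callback damages each hit actor, scaled by the frame's delta time.
; Radius grows by a fixed step per tick up to MaxRadius, so expansion speed depends on frame rate.
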(event `self.ReceiveTick`
  (params (DeltaSeconds :type "Float (single-precision)"))
  (bind _returnvalue (+ (`self.Radius`) 1.0))
  (bind _asbp_main_game_state (cast `/Game/Loadouts/Characters/BaseClass/BP_MainGameState` (`GameplayStatics.GetGameState`)))
  (`/Game/Loadouts/Characters/BaseClass/BP_MainGameState.Spawn AOE` _asbp_main_game_state (`self.K2_GetActorLocation`) (`self.Radius`) false self (delegate `Damage AOE`) 0.1 (struct :`R` 0.064425 :`G` 0.375 :`A` 1.0))
  (if (<= _returnvalue (`self.Max Radius`))
    (set `self.Radius` _returnvalue)))

(event `Damage AOE`
  (params (`Hit Actor` :type "Actor Object Reference"))
  (`GameplayStatics.ApplyDamage` `Hit Actor` (* (stale `self.ReceiveTick` DeltaSeconds) 10.0) null self))

(fn `UserConstructionScript`)