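; BP_Mine is a proximity mine that explodes when an actor implementing BPI_HealthInterface overlaps its Box.
; On trigger it asks BP_MainGameState to spawn an area-of-effect just above its location, passing itself as instigator, then destroys itself.
; Its Explode event is passed as the AOE's hit delegate and applies fixed damage to the hit actor.
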(event `self.Box.OnComponentBeginOverlap`
  (params (OverlappedComponent :type "PrimitiveComponent Object Reference") (OtherActor :type "Actor Object Reference") (OtherComp :type "PrimitiveComponent Object Reference") (OtherBodyIndex :type Integer) (bFromSweep :type Boolean) (SweepResult :type "HitResult Structure (by ref)"))
  (if (`KismetSystemLibrary.DoesImplementInterface` OtherActor "/Game/HealthInterface/BPI_HealthInterface.BPI_HealthInterface_C")
    (bind _asbp_main_game_state (cast `/Game/Loadouts/Characters/BaseClass/BP_MainGameState` (`GameplayStatics.GetGameState`)))
    (`/Game/Loadouts/Characters/BaseClass/BP_MainGameState.Spawn AOE` _asbp_main_game_state (+ (`self.K2_GetActorLocation`) (0.0 0.0 1.0)) 400.0 true self (delegate `Explode`) 2.0 (struct :`A` 1.0))
    (`self.K2_DestroyActor`)))

(event `Explode`
  (params (`Hit Actor` :type "Actor Object Reference"))
  (`GameplayStatics.ApplyDamage` `Hit Actor` 40.0))

(fn `UserConstructionScript`)