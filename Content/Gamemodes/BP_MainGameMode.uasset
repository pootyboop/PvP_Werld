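; Base game mode that handles player spawning, respawning after death and ending the match.
; New and killed players go through PlayerSetup, which waits a second, unpossesses the controller and asks BP_MainGameState to spawn it for the current Gamemode.
; FindSpawnPoint picks random BP_SpawnPoint actors until one is not recently used.
; Win runs once, flagging each tracked player's character as game over and calling EndGameMulti; kill and assist events are empty.
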(event `self.K2_OnLogout`
  (params (ExitingController :type "Controller Object Reference"))
  (`KismetArrayLibrary.Array_RemoveItem` (`self.PCs`) (cast `/Game/Loadouts/Characters/BaseClass/BP_MainPC` ExitingController :!pure true)))

(event `self.HandleStartingNewPlayer`
  (params (NewPlayer :type "PlayerController Object Reference"))
  (`self.Player Setup` NewPlayer))

(event `Player Setup`
  (params (`New Player` :type "PlayerController Object Reference"))
  (bind _asbp_main_pc (cast `/Game/Loadouts/Characters/BaseClass/BP_MainPC` `New Player` :!pure true))
  (`KismetSystemLibrary.Delay` 1.0)
  (`Controller.UnPossess` _asbp_main_pc)
  (`/Game/Loadouts/Characters/BaseClass/BP_MainGameState.Spawn Player` (cast `/Game/Loadouts/Characters/BaseClass/BP_MainGameState` (`GameplayStatics.GetGameState`) :!pure true) (`self.FindSpawnPoint`) _asbp_main_pc (`self.Gamemode`)))

(event `self.ReceiveBeginPlay`)

(event `On Kill`
  (params (Killer :type "/Game/Loadouts/Characters/BaseClass/BP_CharacterBase Object Reference")))

(event `On Kill Assist`
  (params (Assister :type "/Game/Loadouts/Characters/BaseClass/BP_CharacterBase Object Reference")))

(event `Win`
  (params (`Main PlayerState` :type "/Game/Loadouts/Characters/BaseClass/BP_MainPlayerState Object Reference"))
  (if (not (`self.Game Over`))
    (set `self.Game Over` true)
    (for _array_element (`self.PCs`)
      (`|ExecutionSequence`
        (:`then_0`
          (bind _asbp_character_base (cast `/Game/Loadouts/Characters/BaseClass/BP_CharacterBase` (`Controller.K2_GetPawn` _array_element)))
          (set `/Game/Loadouts/Characters/BaseClass/BP_CharacterBase.Game Over` true _asbp_character_base))
        (:`then_1`
          (`/Game/Loadouts/Characters/BaseClass/BP_MainPC.End Game Multi` _array_element `Main PlayerState`))))))

(fn `FindSpawnPoint`
  (returns (ReturnValue :type "Transform Structure (by ref)"))
  (locals (`Spawn Point` :type "/Game/BP_SpawnPoint Object Reference"))
  (bind _spawn_point (`local.Spawn Point`))
  (while true
    (bind _outactors (`GameplayStatics.GetAllActorsOfClass` "/Game/BP_SpawnPoint.BP_SpawnPoint_C"))
    (bind _output_get (set `local.Spawn Point` (`|GetArrayItem` _outactors (`KismetMathLibrary.RandomInteger` (`KismetArrayLibrary.Array_Length` _outactors)))))
    (if (not (`/Game/BP_SpawnPoint.justUsed` _output_get))
      (for _array_element (`PrimitiveComponent.GetOverlappingActors` (`/Game/BP_SpawnPoint.Player Check Collision` (`local.Spawn Point`)) "/Game/Loadouts/Characters/BaseClass/BP_CharacterBase.BP_CharacterBase_C")
        (if (`.bSuccess` (cast `/Game/Loadouts/Characters/BaseClass/BP_CharacterBase` _array_element :!pure true))
          (break)))
      (`/Game/BP_SpawnPoint.Event PlayerSpawn` _spawn_point)
      (return (`self.GetTransform` _spawn_point)))))

(fn `On Player Killed`
  (params (Player :type "PlayerController Object Reference"))
  (locals (Controller :type "Controller Object Reference"))
  (set `local.Controller` Player)
  (`self.Player Setup` Player))

(fn `UserConstructionScript`)