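; Point Control game mode where players score by owning active BP_Point actors, with bonus score for kills and assists.
; A looping timer announces a chat countdown, then swaps in up to three random points, scaled by player count and excluding just-active ones.
; A faster timer awards score to each active point's owner.
; Winning stops both timers and deactivates all points before running parent win logic.
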(event `self.ReceiveBeginPlay`
  (`parent.ReceiveBeginPlay`)
  (`KismetSystemLibrary.Delay` 5.0)
  (`self.Cycle Points`)
  (bind _returnvalue (`KismetSystemLibrary.K2_SetTimerDelegate` (delegate `Cycle Points`) 60.0 true))
  (set `self.Cycle Points Timer` _returnvalue)
  (bind _returnvalue_2 (`KismetSystemLibrary.K2_SetTimerDelegate` (delegate `Grant Points`) 2.0 true))
  (set `self.Grant Points Timer` _returnvalue_2))

(event `Cycle Points`
  (`/Game/BPFunctionLibrary.Send Chat Message` (`|MakeArray` (make `/Game/UI/In-Game/Chat/STextColor` "New points in ") (make `/Game/UI/In-Game/Chat/STextColor` "3" (struct :`R` 1.0 :`G` 1.0 :`A` 1.0)) (make `/Game/UI/In-Game/Chat/STextColor` "...") :!type "/Game/UI/In-Game/Chat/STextColor Structure"))
  (`KismetSystemLibrary.Delay` 1.0)
  (`/Game/BPFunctionLibrary.Send Chat Message` (`|MakeArray` (make `/Game/UI/In-Game/Chat/STextColor` "New points in ") (make `/Game/UI/In-Game/Chat/STextColor` "2" (struct :`R` 1.0 :`G` 1.0 :`A` 1.0)) (make `/Game/UI/In-Game/Chat/STextColor` "...") :!type "/Game/UI/In-Game/Chat/STextColor Structure"))
  (`KismetSystemLibrary.Delay` 1.0)
  (`/Game/BPFunctionLibrary.Send Chat Message` (`|MakeArray` (make `/Game/UI/In-Game/Chat/STextColor` "New points in ") (make `/Game/UI/In-Game/Chat/STextColor` "1" (struct :`R` 1.0 :`G` 0.979 :`A` 1.0)) (make `/Game/UI/In-Game/Chat/STextColor` "...") :!type "/Game/UI/In-Game/Chat/STextColor Structure"))
  (`KismetSystemLibrary.Delay` 1.0)
  (`self.Reset Points` true))

(event `Grant Points`
  (bind _outactors (`GameplayStatics.GetAllActorsOfClass` "/Game/Gamemodes/Point/BP_Point.BP_Point_C"))
  (for _array_element _outactors
    (if (`/Game/Gamemodes/Point/BP_Point.isActive` _array_element)
      (bind _owning_player (`/Game/Gamemodes/Point/BP_Point.Owning Player` _array_element)
        (:`then`
          (bind _asbp_main_player_state (cast `/Game/Loadouts/Characters/BaseClass/BP_MainPlayerState` (`Controller.PlayerState` _owning_player) :!pure true))
          (`/Game/Loadouts/Characters/BaseClass/BP_MainPlayerState.Set Game Score` _asbp_main_player_state (+ (`/Game/Loadouts/Characters/BaseClass/BP_MainPlayerState.Game Score` _asbp_main_player_state) 1.0) _owning_player))
        (:`else`)))))

(event `self.Win`
  (params (`Main PlayerState` :type "/Game/Loadouts/Characters/BaseClass/BP_MainPlayerState Object Reference"))
  (`KismetSystemLibrary.K2_ClearAndInvalidateTimerHandle` (`self.Cycle Points Timer`))
  (`KismetSystemLibrary.K2_ClearAndInvalidateTimerHandle` (`self.Grant Points Timer`))
  (`self.Reset Points` false)
  (`parent.Win` `Main PlayerState`))

(event `self.On Kill`
  (params (Killer :type "/Game/Loadouts/Characters/BaseClass/BP_CharacterBase Object Reference"))
  (bind _asbp_main_player_state (cast `/Game/Loadouts/Characters/BaseClass/BP_MainPlayerState` (`Pawn.PlayerState` Killer) :!pure true))
  (`parent.On Kill` Killer)
  (bind _asbp_main_pc (cast `/Game/Loadouts/Characters/BaseClass/BP_MainPC` (`Pawn.GetController` Killer)))
  (`/Game/Loadouts/Characters/BaseClass/BP_MainPlayerState.Set Game Score` _asbp_main_player_state (+ (`/Game/Loadouts/Characters/BaseClass/BP_MainPlayerState.Game Score` _asbp_main_player_state) 5.0) _asbp_main_pc))

(event `self.On Kill Assist`
  (params (Assister :type "/Game/Loadouts/Characters/BaseClass/BP_CharacterBase Object Reference"))
  (bind _asbp_main_player_state (cast `/Game/Loadouts/Characters/BaseClass/BP_MainPlayerState` (`Pawn.PlayerState` Assister) :!pure true))
  (`parent.On Kill Assist` Assister)
  (bind _asbp_main_pc (cast `/Game/Loadouts/Characters/BaseClass/BP_MainPC` (`Pawn.GetController` Assister)))
  (`/Game/Loadouts/Characters/BaseClass/BP_MainPlayerState.Set Game Score` _asbp_main_player_state (+ (`/Game/Loadouts/Characters/BaseClass/BP_MainPlayerState.Game Score` _asbp_main_player_state) 2.0) _asbp_main_pc))

(fn `Find Random Verified Point`
  (params (Points :type "Array of /Game/Gamemodes/Point/BP_Point Object Reference"))
  (returns (`Verified Point` :type "/Game/Gamemodes/Point/BP_Point Object Reference"))
  (locals (`Current Point` :type "/Game/Gamemodes/Point/BP_Point Object Reference"))
  (bind _current_point (`local.Current Point`))
  (while true
    (set `local.Current Point` (`KismetArrayLibrary.Array_Random` Points))
    (if (`KismetMathLibrary.BooleanNOR` (`/Game/Gamemodes/Point/BP_Point.isActive` _current_point) (`/Game/Gamemodes/Point/BP_Point.wasActive` _current_point))
      (return (`local.Current Point`)))))

(fn `Reset Points`
  (params (`Activate New Points` :type Boolean))
  (locals (Points :type "Array of /Game/Gamemodes/Point/BP_Point Object Reference") (PointCt :type Integer :default 0))
  (`|ExecutionSequence`
    (:`then_0`
      (bind _outactors (`GameplayStatics.GetAllActorsOfClass` "/Game/Gamemodes/Point/BP_Point.BP_Point_C"))
      (bind _output_get (set `local.Points` _outactors))
      (for _array_element _output_get
        (set `/Game/Gamemodes/Point/BP_Point.wasActive` false _array_element)
        (if (`/Game/Gamemodes/Point/BP_Point.isActive` _array_element)
          (set `/Game/Gamemodes/Point/BP_Point.wasActive` true _array_element))
        (`/Game/Gamemodes/Point/BP_Point.Change Is Active State` _array_element false false))
      (if `Activate New Points`
        (bind _outactors_2 (`GameplayStatics.GetAllActorsOfClass` "/Script/Engine.PlayerController"))
        (bind _returnvalue (- (`KismetArrayLibrary.Array_Length` _outactors_2) 1))
        (set `local.PointCt` (`KismetMathLibrary.SelectInt` 3 _returnvalue (>= _returnvalue 4)))
        (while (> (`local.PointCt`) 0)
          (`/Engine/EditorBlueprintResources/StandardMacros.DecrementInt` (`local.PointCt`)
            (:`  `
              (`/Game/Gamemodes/Point/BP_Point.Change Is Active State` (`self.Find Random Verified Point` (`local.Points`)) true false))))))
    (:`then_1`
      (if `Activate New Points`
        (`/Game/BPFunctionLibrary.Send Chat Message` (`|MakeArray` (make `/Game/UI/In-Game/Chat/STextColor` "New points!" (struct :`R` 1.0 :`G` 1.0 :`A` 1.0)) :!type "/Game/UI/In-Game/Chat/STextColor Structure"))))))

(fn `UserConstructionScript`
  (`parent.UserConstructionScript`))