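; BP_Point is a capture point actor for a game mode, taken when a character overlaps its mesh.
; A new owner triggers a chat message and crosshair notice, and the point takes that character's color through a dynamic material and W_Point widget.
; ChangeIsActiveState routes through a Multi event to toggle visibility, collision and tick, clearing owner and color to grey when inactive.
; Tick checks overlapping characters against the owner but takes no action.
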(event `self.ReceiveBeginPlay`
  (bind _asw_point (cast `/Game/Gamemodes/Point/W_Point` (`WidgetComponent.GetWidget` (`self.Widget`)) :!pure true))
  (`self.Change Is Active State` (`self.isActive`))
  (`/Game/Gamemodes/Point/W_Point.Set Color` _asw_point (`self.Color`))
  (`/Game/Gamemodes/Point/W_Point.Set Name` _asw_point (`self.Name`)))

(event `self.Point Mesh.OnComponentBeginOverlap`
  (params (OverlappedComponent :type "PrimitiveComponent Object Reference") (OtherActor :type "Actor Object Reference") (OtherComp :type "PrimitiveComponent Object Reference") (OtherBodyIndex :type Integer) (bFromSweep :type Boolean) (SweepResult :type "HitResult Structure (by ref)"))
  (bind _asbp_character_base (cast `/Game/Loadouts/Characters/BaseClass/BP_CharacterBase` OtherActor))
  (`self.Point Taken` (cast `/Game/Loadouts/Characters/BaseClass/BP_MainPC` (`Pawn.GetController` _asbp_character_base) :!pure true)))

(event `Change isActive State Multi`
  (params (isActive :type Boolean))
  (`self.Change Is Active State` isActive true))

(event `self.ReceiveTick`
  (params (DeltaSeconds :type "Float (single-precision)"))
  (bind _overlappingactors (`PrimitiveComponent.GetOverlappingActors` (`self.Point Mesh`) "/Game/Loadouts/Characters/BaseClass/BP_CharacterBase.BP_CharacterBase_C"))
  (if (!= (`KismetArrayLibrary.Array_Length` _overlappingactors) 0)
    (for _array_element _overlappingactors
      (bind _asbp_character_base (cast `/Game/Loadouts/Characters/BaseClass/BP_CharacterBase` _array_element))
      (if (== (`Pawn.GetController` _asbp_character_base) (`self.Owning Player`))
        _))))

(event `Point Taken`
  (params (`Owning Player` :type "/Game/Loadouts/Characters/BaseClass/BP_MainPC Object Reference"))
  (`/Engine/EditorBlueprintResources/StandardMacros.IsValid` `Owning Player`
    (:`Is Valid`
      (if (!= `Owning Player` (`self.Owning Player`))
        (bind _output_get (set `self.Owning Player` `Owning Player`))
        (bind _asbp_main_player_state (cast `/Game/Loadouts/Characters/BaseClass/BP_MainPlayerState` (`Controller.PlayerState` _output_get) :!pure true))
        (`/Game/BPFunctionLibrary.Send Chat Message` (`|MakeArray` (make `/Game/UI/In-Game/Chat/STextColor` (`KismetTextLibrary.Conv_StringToText` (`/Game/Loadouts/Characters/BaseClass/BP_MainPlayerState.Player Name` _asbp_main_player_state)) (`/Game/Loadouts/Characters/BaseClass/BP_MainPlayerState.Color` _asbp_main_player_state)) (make `/Game/UI/In-Game/Chat/STextColor` " took ") (make `/Game/UI/In-Game/Chat/STextColor` (`KismetTextLibrary.Conv_StringToText` (`self.Name`))) (make `/Game/UI/In-Game/Chat/STextColor` "!") :!type "/Game/UI/In-Game/Chat/STextColor Structure"))
        (bind _owning_player (`self.Owning Player`)
          (:`then`
            (bind _asbp_character_base (cast `/Game/Loadouts/Characters/BaseClass/BP_CharacterBase` (`Controller.K2_GetPawn` _owning_player)))
            (bind _color (`/Game/Loadouts/Characters/BaseClass/BP_CharacterBase.Color` _asbp_character_base))
            (`self.Set Point Color Multi` _color)
            (`/Game/Loadouts/Characters/BaseClass/BP_CharacterBase.Crosshair Info` _asbp_character_base (`KismetTextLibrary.Conv_StringToText` (`KismetStringLibrary.Concat_StrStr` "Took Point " (`self.Name`) "!")) _color))
          (:`else`))))))

(event `Set Point Color Multi`
  (params (Color :type "LinearColor Structure"))
  (`self.Set Point Color` Color))

(fn `Change Is Active State`
  (params (isActive :type Boolean) (Multicast :type Boolean))
  (bind _defaultsceneroot (`self.DefaultSceneRoot`))
  (if Multicast
    (bind _output_get (set `self.isActive` isActive))
    (`SceneComponent.SetHiddenInGame` (`self.DefaultSceneRoot`) (not _output_get) true)
    (`PrimitiveComponent.SetCollisionEnabled` (`self.Point Mesh`) (select `bool` _output_get :`false` "NoCollision" :`true` "QueryAndPhysics" :!type "ECollisionEnabled Enum"))
    (`self.SetActorTickEnabled` _output_get)
    (if _output_get
      (`ActorComponent.Activate` _defaultsceneroot false)
      (else
        (set `self.Owning Player` null)
        (`self.Set Point Color Multi` (struct :`R` 0.5 :`G` 0.5 :`B` 0.5 :`A` 1.0))
        (`ActorComponent.Deactivate` _defaultsceneroot)))
    (else
      (`self.Change isActive State Multi` isActive))))

(fn `Set Point Color`
  (params (Color :type "LinearColor Structure"))
  (bind _output_get (set `self.Color` Color))
  (`MaterialInstanceDynamic.SetVectorParameterValue` (`self.Dynamic Material Inst`) "Color" _output_get)
  (`/Game/Gamemodes/Point/W_Point.Set Color` (cast `/Game/Gamemodes/Point/W_Point` (`WidgetComponent.GetWidget` (`self.Widget`)) :!pure true) (`local.Color`)))

(fn `UserConstructionScript`
  (bind _returnvalue (`KismetMaterialLibrary.CreateDynamicMaterialInstance` "/Game/Gamemodes/Point/M_Point_Inst.M_Point_Inst" "M_Point_DynamicInst"))
  (bind _output_get (set `self.Dynamic Material Inst` _returnvalue))
  (`PrimitiveComponent.SetMaterial` (`self.Point Mesh`) 0 _output_get)
  (`MaterialInstanceDynamic.SetVectorParameterValue` (`self.Dynamic Material Inst`) "Color" (`self.Color`)))