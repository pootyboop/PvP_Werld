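; Lobby game mode that runs a two-map vote and moves to the winning level once every player is ready.
; BeginPlay picks two distinct random maps from a hardcoded list.
; A map of player controllers to votes tracks readiness, with -1 meaning undecided, and is rechecked on each ReadyUp or logout.
; When all have voted, it tallies votes, favors Map1 on ties, and opens the level through SteamGameInstance.
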(event `self.ReceiveBeginPlay`
  (bind (_map1 _map2) (`self.Get Two Random Maps`))
  (set `self.Map1` _map1)
  (set `self.Map2` _map2))

(event `self.K2_PostLogin`
  (params (NewPlayer :type "PlayerController Object Reference"))
  (`parent.K2_PostLogin` NewPlayer)
  (`BlueprintMapLibrary.Map_Add` (`self.Lobby PCs`) (cast `/Game/Loadouts/Characters/BaseClass/BP_MainPC` NewPlayer :!pure true) -1))

(event `self.K2_OnLogout`
  (params (ExitingController :type "Controller Object Reference"))
  (`BlueprintMapLibrary.Map_Remove` (`self.Lobby PCs`) (cast `/Game/Loadouts/Characters/BaseClass/BP_MainPC` ExitingController :!pure true))
  (`self.Check if Ready to Start`))

(event `Ready Up`
  (params (`Main PC` :type "/Game/Loadouts/Characters/BaseClass/BP_MainPC Object Reference") (`Map Vote` :type "Integer (by ref)"))
  (`BlueprintMapLibrary.Map_Add` (`self.Lobby PCs`) `Main PC` `Map Vote`)
  (`self.Check if Ready to Start`))

(event `Check if Ready to Start`
  (if (`self.Ready to Start`)
    (`self.Open Most Voted Level`)))

(fn `Get Two Random Maps`
  (returns (Map1 :type String) (Map2 :type String))
  (locals (`Map 1` :type String) (`Map 2` :type String))
  (bind _output_get (set `local.Map 1` (`KismetArrayLibrary.Array_Random` (`|MakeArray` "CloudIslands" "DownyDistrict" "ReplicationTestLevel"))))
  (set `local.Map 2` _output_get)
  (while (`KismetStringLibrary.EqualEqual_StrStr` (`local.Map 1`) (`local.Map 2`))
    (set `local.Map 2` (`KismetArrayLibrary.Array_Random` (`|MakeArray` "CloudIslands" "DownyDistrict" "ReplicationTestLevel"))))
  (return (`local.Map 1`) (`local.Map 2`)))

(fn `Open Most Voted Level`
  (locals (`Map1 Votes` :type Integer) (`Map2 Votes` :type Integer) (`Map to Open` :type String))
  (bind _values (`BlueprintMapLibrary.Map_Values` (`self.Lobby PCs`)))
  (for _array_element _values
    (if (== _array_element 1)
      (`/Engine/EditorBlueprintResources/StandardMacros.IncrementInt` (`local.Map1 Votes`))
      (elif (== _array_element 2)
        (`/Engine/EditorBlueprintResources/StandardMacros.IncrementInt` (`local.Map2 Votes`)))))
  (`BlueprintMapLibrary.Map_Clear` (`self.Lobby PCs`))
  (`|ExecutionSequence`
    (:`then_0`
      (if (>= (`local.Map1 Votes`) (`local.Map2 Votes`))
        (set `local.Map to Open` (`self.Map1`))
        (else
          (set `local.Map to Open` (`self.Map2`)))))
    (:`then_1`
      (`/Game/SteamAndMenu/SteamGameInstance.Open Level` (cast `/Game/SteamAndMenu/SteamGameInstance` (`GameplayStatics.GetGameInstance`) :!pure true) (`local.Map to Open`)))))

(fn `Ready to Start`
  (returns (Return :type Boolean))
  (bind _lobby_pcs (`self.Lobby PCs`))
  (bind _keys (`BlueprintMapLibrary.Map_Keys` _lobby_pcs))
  (bind _values (`BlueprintMapLibrary.Map_Values` _lobby_pcs))
  (for (_ _array_index) _keys
    (if (not (!= (`|GetArrayItem` _values _array_index) -1))
      (return false)))
  (return true))

(fn `UserConstructionScript`
  (`parent.UserConstructionScript`))